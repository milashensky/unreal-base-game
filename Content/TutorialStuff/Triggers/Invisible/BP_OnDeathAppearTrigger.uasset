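; Tutorial trigger that makes a set of hidden actors appear at its own location, presumably on a death, as its name suggests.
; Its TriggerAction override calls the parent, then unhides and teleports each Appearing actor to the trigger before destroying itself.
; The tick and collision enable calls in that loop target the trigger itself, not the appearing actors.
; The BeginPlay loop over Appearing has an empty body.
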(event EventBeginPlay
  (|CallParentFunction)
  (for _array_element (Variables|Default|GetAppearing)
    _))

(event Collision|EventActorBeginOverlap
  (params (OtherActor :type Actor%20Object%20Reference))
  (|CallParentFunction OtherActor) ; This node is disabled and will not be called.\nDrag off pins to build functionality.
)

(event EventTick
  (params (DeltaSeconds :type Float%20%28single-precision%29))
  (|CallParentFunction DeltaSeconds) ; This node is disabled and will not be called.\nDrag off pins to build functionality.
)

(fn ConstructionScript
  (|CallParentFunction))

(fn TriggerAction
  (|CallParentFunction)
  (for _array_element (Variables|Default|GetAppearing)
    (Rendering|SetActorHiddenInGame _array_element false)
    (Actor|Tick|SetActorTickEnabled true)
    (Collision|SetActorEnableCollision true)
    (Transformation|SetActorLocation _array_element (Transformation|GetActorLocation) false true))
  (Actor|DestroyActor))