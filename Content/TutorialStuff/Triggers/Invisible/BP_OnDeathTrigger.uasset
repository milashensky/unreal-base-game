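; BP_OnDeathTrigger is a tutorial trigger that fires an action once every actor in its ShouldDie list is dead.
; On BeginPlay it gets each listed actor's health component through a message call and binds to its OnDeath event.
; Each death runs CheckAllDead, which polls every actor's dead state and calls TriggerAction when all are dead.
; TriggerAction is empty in this Blueprint.
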(event Custom|OnActorDeath
  (params (Damage :type S%20Damage%20Info%20Structure))
  (bind _isalldead (CallFunction|CheckAllDead))
  (if _isalldead
    (CallFunction|TriggerAction)))

(event EventBeginPlay
  (for _array_element (Variables|Default|GetShouldDie)
    (bind _healthcomponent (Class|PBIDamageable|GetHealthComponent(Message) _array_element))
    (Utilities|IsValid _healthcomponent
      (:Is%20Valid
        (EventDispatchers|AssignOnDeath _healthcomponent (delegate Custom|OnActorDeath))))))

(event Collision|EventActorBeginOverlap
  (params (OtherActor :type Actor%20Object%20Reference)))

(event EventTick
  (params (DeltaSeconds :type Float%20%28single-precision%29)))

(fn ConstructionScript)

(fn CheckAllDead
  (for _array_element (Variables|Default|GetShouldDie)
    (bind _isdead (Class|PBIDamageable|GetIsDead(Message) _array_element))
    (if (not _isdead)
      (return false)))
  (return true))

(fn TriggerAction)