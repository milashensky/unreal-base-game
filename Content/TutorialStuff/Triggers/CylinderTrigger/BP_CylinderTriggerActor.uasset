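; Cylinder trigger actor in the tutorial content that reacts when an actor tagged Player enters it.
; Sphere begin-overlap calls TriggerAction while IsActive is set; TriggerAction is an empty hook here.
; SetActiveState stores the flag and toggles actor visibility plus the Cylinder's visibility, activation and collision, leaving the Sphere's collision untouched.
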(event OnComponentBeginOverlap(Sphere)
  (params (OverlappedComponent :type Primitive%20Component%20Object%20Reference) (OtherActor :type Actor%20Object%20Reference) (OtherComp :type Primitive%20Component%20Object%20Reference) (OtherBodyIndex :type Integer) (bFromSweep :type Boolean) (SweepResult :type Hit%20Result%20Structure%20%28by%20ref%29))
  (if (Variables|Default|GetIsActive)
    (if (Actor|ActorHasTag OtherActor "Player")
      (CallFunction|TriggerAction))))

(event EventBeginPlay)

(event Collision|EventActorBeginOverlap
  (params (OtherActor :type Actor%20Object%20Reference)))

(event EventTick
  (params (DeltaSeconds :type Float%20%28single-precision%29)))

(fn ConstructionScript)

(fn SetActiveState
  (params (IsActive :type Boolean))
  (bind _cylinder (Variables|Default|GetCylinder))
  (bind _output_get (Variables|Default|SetIsActive IsActive))
  (Rendering|SetVisibility _cylinder IsActive true)
  (Components|Activation|SetActive _cylinder IsActive true)
  (Rendering|SetActorHiddenInGame (not _output_get))
  (if IsActive
    (Collision|SetCollisionEnabled (Variables|Default|GetCylinder) "QueryAndPhysics")
    (else
      (Collision|SetCollisionEnabled (Variables|Default|GetCylinder) "NoCollision"))))

(fn TriggerAction)