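; BP_WoodenBow is a wooden bow weapon Blueprint that reports itself as ranged.
; Its ShootProjectile event spawns the given projectile class at the ProjectileSpawnPos transform, always spawning regardless of collision, with the owner as instigator.
; It then passes the bow's base damage from DamageInfo to the spawned projectile through a SetWeaponBaseDamage message.
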(event EventBeginPlay
  (|CallParentFunction) ; This node is disabled and will not be called.\nDrag off pins to build functionality.
)

(event Collision|EventActorBeginOverlap
  (params (OtherActor :type Actor%20Object%20Reference))
  (|CallParentFunction OtherActor) ; This node is disabled and will not be called.\nDrag off pins to build functionality.
)

(event EventTick
  (params (DeltaSeconds :type Float%20%28single-precision%29))
  (|CallParentFunction DeltaSeconds) ; This node is disabled and will not be called.\nDrag off pins to build functionality.
)

(event EventShootProjectile
  (params (Owner :type Pawn%20Object%20Reference) (Projectile :type Actor%20Class%20Reference))
  (bind _projectilespawnpos (Variables|Default|GetProjectileSpawnPos))
  (bind _returnvalue (Transformation|GetWorldTransform _projectilespawnpos))
  (bind _returnvalue_2 (Game|SpawnActorfromClass Projectile (Math|Transform|MakeTransform (.location _returnvalue) (.rotation _returnvalue) (.scale _returnvalue)) "AlwaysSpawn" "MultiplyWithRoot" 0 Owner))
  (Class|BPIProjectile|SetWeaponBaseDamage(Message) _returnvalue_2 (.basedamage (Variables|Default|GetDamageInfo))))

(fn ConstructionScript
  (|CallParentFunction))

(fn GetIsRanged
  (return true))