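; Base weapon actor for melee attacks, providing hit detection, getters for weapon stats and a physics-based drop.
; StartAttack and EndAttack clear the hit-actor set and spawn or destroy a Niagara trail sized from the hit box.
; HitDetect box-traces at the hit box, ignoring owner and prior hits, and rejects hits behind WorldStatic walls using a line trace.
; Construction derives range from the hit box extent when range is zero.
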(event Collision|EventActorBeginOverlap
  (params (OtherActor :type Actor%20Object%20Reference)))

(event EventTick
  (params (DeltaSeconds :type Float%20%28single-precision%29)))

(event EventStartAttack
  (CallFunction|ResetHitActors)
  (CallFunction|SpawnTrailEffect))

(event EventEndAttack
  (CallFunction|ResetHitActors)
  (CallFunction|DespawnTrailEffect))

(fn ConstructionScript
  (CallFunction|AutoSetRange))

(fn CheckCanHitActor
  (params (Actor :type Actor%20Object%20Reference%20%28by%20ref%29))
  (return (not (Utilities|Set|Contains (Variables|Default|GetHitActors) Actor))))

(fn ResetHitActors
  (Utilities|Set|Clear (Variables|Default|GetHitActors)))

(fn RegisterHitActor
  (params (NewItem :type Actor%20Object%20Reference%20%28by%20ref%29))
  (Utilities|Set|Add (Variables|Default|GetHitActors) NewItem))

(fn GetIgnoredHitActors
  (bind _returnvalue (Components|GetOwner))
  (Utilities|FlowControl|Sequence
    (:then_0
      (Utilities|IsValid _returnvalue
        (:Is%20Valid
          (LocalVariables|SetOwnerActor _returnvalue))))
    (:then_1
      (bind _result (Utilities|Set|ToArray (Variables|Default|GetHitActors)))
      (bind _output_get (LocalVariables|SetIgnoredActorsLoc _result))
      (Utilities|Array|Add _output_get (LocalVariables|GetOwnerActor))
      (return (LocalVariables|GetIgnoredActorsLoc)))))

(fn AutoSetRange
  (if (== (Variables|Default|GetWeaponRange) 0.0)
    (Variables|Default|SetWeaponRange (* (Math|Vector|VectorLength (Variables|/Script/Engine.BoxComponent|GetBoxExtent (Variables|Default|GetHitBox))) 2.0))))

(fn SpawnTrailEffect
  (bind _traileffectsystem (Variables|Params|GetTrailEffectSystem))
  (Utilities|IsValid _traileffectsystem
    (:Is%20Valid
      (bind _returnvalue (Niagara|SpawnSystemAttached _traileffectsystem (Variables|Default|GetTrailEffectLocation) "None" "0, 0, 0" "0, 0, 0" "KeepRelativeOffset" false))
      (Variables|Default|SetTrailEffectRef _returnvalue)
      (Niagara|SetNiagaraVariable(Float) (Variables|Default|GetTrailEffectRef) "User.Width" (Math|Vector|VectorLength (Components|Box|GetScaledBoxExtent (Variables|Default|GetHitBox)))))))

(fn DespawnTrailEffect
  (bind _traileffectref (Variables|Default|GetTrailEffectRef))
  (Utilities|IsValid _traileffectref
    (:Is%20Valid
      (Components|DestroyComponent _traileffectref))))

(fn CheckIsHittingWall
  (params (HitLocation :type Vector))
  (Utilities|IsValid (Components|GetOwner)
    (:Is%20Valid
      (bind _returnvalue (Collision|LineTraceForObjects (Transformation|GetActorLocation) HitLocation (Utilities|Array|MakeArray "ObjectTypeQuery1") false 0 "None"))
      (return _returnvalue))
    (:Is%20Not%20Valid
      (return false))))

(fn DropItem
  (bind _mesh (Variables|Default|GetMesh))
  (Utilities|FlowControl|Sequence
    (:then_0
      (Collision|SetCollisionObjectType _mesh "ECC_WorldDynamic"))
    (:then_1
      (Collision|SetCollisionEnabled _mesh "PhysicsOnly"))
    (:then_2
      (Physics|SetSimulatePhysics _mesh true))
    (:then_3
      (return true))))

(fn GetAnimSpeed
  (return (Variables|Params|GetAttackAnimRate)))

(fn GetDamageInfo
  (return (Variables|Params|GetDamageInfo)))

(fn GetHitBox
  (return (Variables|Default|GetHitBox)))

(fn GetRange
  (return (Variables|Default|GetWeaponRange)))

(fn GetWeaponType
  (return (Variables|Params|GetType)))

(fn HitDetect
  (bind _hitbox (Variables|Default|GetHitBox))
  (bind _returnvalue (Transformation|GetWorldLocation _hitbox))
  (bind _ignoredactors (CallFunction|GetIgnoredHitActors))
  (bind (_outhit _returnvalue_2) (Class|KismetSystemLibrary|BoxTraceSingleforObjects _returnvalue _returnvalue (Components|Box|GetScaledBoxExtent _hitbox) (Transformation|GetWorldRotation _hitbox) (Utilities|Array|MakeArray "ObjectTypeQuery3" "ObjectTypeQuery4" "ObjectTypeQuery2") false _ignoredactors "None" true))
  (if _returnvalue_2
    (bind _ishittingwall (CallFunction|CheckIsHittingWall (.ImpactPoint (Collision|BreakHitResult _outhit))))
    (if _ishittingwall
      (return "" false)
      (else
        (CallFunction|RegisterHitActor (.HitActor (Collision|BreakHitResult _outhit)))
        (return _outhit _returnvalue_2)))
    (else
      (return "" false))))