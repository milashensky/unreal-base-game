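; Arrow projectile that damages what it hits with a weapon-supplied base damage, ignoring its instigator while moving.
; When it stops, it sends a damage message to the hit actor and reports an AI damage event.
; If damage registers, a component trace finds the bone and embeds the arrow unless the angle is too glancing.
; Otherwise it becomes a loose physics object; either way it destroys itself after a delay.
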(event OnProjectileStop(ProjectileMovement)
  (params (ImpactResult :type Hit%20Result%20Structure%20%28by%20ref%29))
  (bind _collision (Variables|Default|GetCollision))
  (Utilities|FlowControl|Sequence
    (:then_0
      ;[0.15 0.15 0.15 0.5] Change behaviour after hit
      (bind _wasdamaged (Weapon|RegisterDamage (.hitactor ImpactResult) (.impactpoint ImpactResult)))
      (if _wasdamaged
        (bind _isattached (CallFunction|AttachtotheBone (.hitcomponent ImpactResult)))
        (if (not _isattached)
          (Utilities|FlowControl|Sequence :!label _label
            (:then_0
              (Collision|SetCollisionObjectType _collision "ECC_WorldDynamic"))
            (:then_1
              (Collision|SetCollisionEnabled _collision "PhysicsOnly"))
            (:then_2
              (Physics|SetSimulatePhysics _collision true))))
        (else
          (goto _label))))
    (:then_1
      (CallFunction|ScheduleDestory))))

(event Custom|ScheduleDestory
  (Utilities|FlowControl|Delay 6e+01)
  (Actor|DestroyActor))

(event EventBeginPlay
  (bind _returnvalue (Game|GetInstigator))
  (Utilities|IsValid _returnvalue
    (:Is%20Valid
      (Collision|IgnoreActorwhenMoving (Variables|Default|GetCollision) _returnvalue true))))

(event Collision|EventActorBeginOverlap
  (params (OtherActor :type Actor%20Object%20Reference)))

(event EventTick
  (params (DeltaSeconds :type Float%20%28single-precision%29)))

(event EventSetWeaponBaseDamage
  (params (BaseDamage :type Integer))
  (Variables|Default|SetOwnerBaseDamage BaseDamage))

(fn ConstructionScript)

(fn RegisterDamage
  (params (DamagedActor :type Object%20Object%20Reference) (DamageLocation :type Vector))
  (bind _wasdamaged (Class|PBIDamageable|TakeDamage(Message) DamagedActor (Utilities|Struct|MakeS_DamageInfo (Variables|Default|GetOwnerBaseDamage) DamageLocation)))
  (Class|AISenseDamage|ReportDamageEvent 0 (Game|GetInstigator) (Math|Conversions|ToFloat(Integer) (Variables|Default|GetOwnerBaseDamage)) DamageLocation "0, 0, 0" "None")
  (return _wasdamaged))

(fn AttachtotheBone
  (params (TargetComponent :type Primitive%20Component%20Object%20Reference))
  (bind _collision (Variables|Default|GetCollision))
  (bind _staticmesh (Variables|Default|GetStaticMesh))
  (bind (_min _max) (Components|StaticMesh|GetLocalBounds _staticmesh))
  (bind _returnvalue (Transformation|GetWorldLocation _collision))
  (Utilities|IsValid TargetComponent
    (:Is%20Valid
      ;[0.15 0.15 0.15 0.5] Trace For Bone
      (bind (_hitlocation _hitnormal _bonename _outhit _returnvalue_2) (Collision|LineTraceComponent TargetComponent _returnvalue (+ _returnvalue (* (Math|Vector|GetForwardVector _collision) (Math|Vector|VectorLength (Components|Box|GetScaledBoxExtent _collision)) 2)) false false false))
      (LocalVariables|SetHitLocation _hitlocation)
      (LocalVariables|SetHitNormal _hitnormal)
      (LocalVariables|SetTargetBoneName _bonename)
      ;[0.15 0.15 0.15 0.5] IF no bone hit - do nothing
      (if _returnvalue_2
        (if (== (LocalVariables|GetTargetBoneName) "")
          (return false)
          (else
            ;[0.15 0.15 0.15 0.5] If hit angle is not perpendicular enough, do not attach
            (if (> (Math|Float|Absolute(Float) (Math|Vector|DotProduct (LocalVariables|GetHitNormal) (Transformation|GetActorForwardVector))) 0.5)
              ;[0.15 0.15 0.15 0.5] Attach to the bone
              (Collision|SetActorEnableCollision false)
              (Physics|SetSimulatePhysics (Variables|Default|GetCollision) false)
              (bind _returnvalue_3 (Transformation|AttachComponentToComponent TargetComponent (LocalVariables|GetTargetBoneName) "KeepWorld" "KeepWorld" "KeepWorld" true))
              (if _returnvalue_3
                ;[0.15 0.15 0.15 0.5] Set penetration depth
                (bind _returnvalue_4 (Transformation|SetActorLocation (+ (LocalVariables|GetHitLocation) (* (Transformation|GetActorForwardVector) (* (+ (Math|Float|Absolute(Float) (- (.x _min) (.x _max))) (Math|Random|RandomFloatinRange -1.0 1.0)) -0.5))) false false))
                (return _returnvalue_4)
                (else
                  (return false)))
              (else
                (return false)))))
        (else
          (return false))))
    (:Is%20Not%20Valid
      (return false))))

(fn GetProjectileSpeed
  (return (/ (+ (Variables|/Script/Engine.ProjectileMovementComponent|GetMaxSpeed (Variables|Default|GetProjectileMovement)) (Variables|/Script/Engine.ProjectileMovementComponent|GetInitialSpeed (Variables|Default|GetProjectileMovement))) 2.0)))