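; Wolf character Blueprint that deals bite damage through a weapon child actor on its Jaw component.
; Start and end hit-detect events forward interface messages to the Jaw actor to open and close the attack.
; The HandleHitDetect override calls the parent, polls the Jaw for a hit, ignores self, and applies the weapon's base damage by interface message.
; Each hit is also reported to AI perception as a damage event.
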(event EventBeginPlay)

(event Collision|EventActorBeginOverlap
  (params (OtherActor :type Actor%20Object%20Reference)))

(event EventStartHitDetect
  (bind _jaw (Variables|Default|GetJaw))
  (bind _childactor (Variables|/Script/Engine.ChildActorComponent|GetChildActor _jaw))
  ;[0.15 0.15 0.15 0.5] Weapon Hit Detection
  (Utilities|IsValid _childactor
    (:Is%20Valid
      (Class|BPIWeapon|StartAttack(Message) _childactor))))

(event EventTick
  (params (DeltaSeconds :type Float%20%28single-precision%29)))

(event EventEndHitDetect
  (bind _jaw (Variables|Default|GetJaw))
  (bind _childactor (Variables|/Script/Engine.ChildActorComponent|GetChildActor _jaw))
  ;[0.15 0.15 0.15 0.5] Weapon Hit Detection
  (Utilities|IsValid _childactor
    (:Is%20Valid
      (Class|BPIWeapon|EndAttack(Message) _childactor))))

(fn ConstructionScript)

(fn HandleHitDetect
  (bind _jaw (Variables|Default|GetJaw))
  (bind _childactor (Variables|/Script/Engine.ChildActorComponent|GetChildActor _jaw))
  (|CallParentFunction)
  (Utilities|IsValid _childactor
    (:Is%20Valid
      (bind (_hit _ishit) (Class|BPIWeapon|HitDetect(Message) _childactor))
      (if _ishit
        (if (not (== (.hitactor _hit) self))
          (bind _damageinfo (Class|BPIWeapon|GetDamageInfo(Message) _childactor))
          (Class|PBIDamageable|TakeDamage(Message) (.hitactor _hit) (Utilities|Struct|MakeS_DamageInfo (.basedamage _damageinfo) (.location _hit)))
          (Class|AISenseDamage|ReportDamageEvent (.hitactor _hit) self (Math|Conversions|ToFloat(Integer) (.basedamage _damageinfo)) (Transformation|GetActorLocation) (.location _hit) "None"))))))