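; Base humanoid character that adds armed sword, spear and bow combat to its parent character class.
; Weapons are child actors in hand and sheath slots, swapped by SheathingComponent, with a scheduled draw following a sheathe.
; Weapon messages handle hit detection, damage and arrow shooting, while AttackSystem takes attacks and speed from the applied weapon and doubles turn rate during attacks.
; Damage triggers procedural hit reactions, and death also drops held items.
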(event OnWeaponSheathed(SheathingComponent)
  ;[0.15 0.15 0.15 0.5] Sheathing scheduling
  (CallFunction|DrawWeapon (Variables|Default|GetDrawWeaponScheduled)))

(event OnWeaponChangeDone(SheathingComponent)
  (params (IsSuccessful :type Boolean))
  ;[0.15 0.15 0.15 0.5] Sheathing scheduling
  (CallFunction|UpdateSenseSocketUsage)
  (if (not IsSuccessful)
    (Variables|Default|SetDrawWeaponScheduled "NewEnumerator3")))

(event OnAttackStart(AttackSystem)
  (params (Attack :type S%20Attack%20Info%20Structure))
  ;[0.15 0.15 0.15 0.5] AttackComponent
  (Variables|/Script/Engine.CharacterMovementComponent|SetRotationRate (Variables|Character|GetCharacterMovement) (* (Variables|Components|GetDefaultTurnRate) 2.0)))

(event OnAttackEnd(AttackSystem)
  ;[0.15 0.15 0.15 0.5] AttackComponent
  (AttackSystem|HandleAttackEnd))

(event EventLoadProjectile
  (ChildActorComponent|SetChildActorClass (Variables|Default|GetArrowSlot) (Variables|WeaponData|GetBowArrowClass)))

(event EventEndHitDetect
  (bind _righthandweaponslot (Variables|WeaponSlots|GetRightHandWeaponSlot))
  (bind _childactor (Variables|/Script/Engine.ChildActorComponent|GetChildActor _righthandweaponslot))
  ;[0.15 0.15 0.15 0.5] AttackComponent
  ;;[0.15 0.15 0.15 0.5] Weapon Hit Detection
  (Utilities|IsValid _childactor
    (:Is%20Valid
      (Class|BPIWeapon|EndAttack(Message) _childactor))))

(event EventStartHitDetect
  (bind _righthandweaponslot (Variables|WeaponSlots|GetRightHandWeaponSlot))
  (bind _childactor (Variables|/Script/Engine.ChildActorComponent|GetChildActor _righthandweaponslot))
  ;[0.15 0.15 0.15 0.5] AttackComponent
  ;;[0.15 0.15 0.15 0.5] Weapon Hit Detection
  (Utilities|IsValid _childactor
    (:Is%20Valid
      (Class|BPIWeapon|StartAttack(Message) _childactor))))

(fn ConstructionScript)

(fn CanParkour
  (bind _canperform (Default|GetHasEnoughStaminaforAction (Variables|Default|GetStaminaComponent) (Variables|Default|GetJumpStaminaCostValue)))
  (return _canperform))

(fn CanChangeWeapon
  (if (Class|AnimInstance|IsAnyMontagePlaying (Components|SkeletalMesh|GetAnimInstance (Variables|Character|GetMesh)))
    (return false)
    (else
      (bind _isattacking (CallFunction|GetIsAttacking))
      (if _isattacking
        (return false)
        (else
          (return (AI|Components|NavMovement|IsMovingonGround (Variables|Character|GetCharacterMovement))))))))

(fn GetArmedWeaponSlot
  (bind _lefthandweaponslot (Variables|WeaponSlots|GetLeftHandWeaponSlot))
  (bind _righthandweaponslot (Variables|WeaponSlots|GetRightHandWeaponSlot))
  (Utilities|IsValid _lefthandweaponslot
    (:Is%20Valid
      (Utilities|IsValid (Variables|/Script/Engine.ChildActorComponent|GetChildActor _lefthandweaponslot)
        (:Is%20Valid
          (return (Variables|WeaponSlots|GetLeftHandWeaponSlot)))
        (:Is%20Not%20Valid
          _)))
    (:Is%20Not%20Valid
      _))
  (Utilities|IsValid _righthandweaponslot
    (:Is%20Valid
      (Utilities|IsValid (Variables|/Script/Engine.ChildActorComponent|GetChildActor _righthandweaponslot)
        (:Is%20Valid
          (return (Variables|WeaponSlots|GetRightHandWeaponSlot)))
        (:Is%20Not%20Valid
          _)))
    (:Is%20Not%20Valid
      _))
  (return 0))

(fn GetWeaponArmSlot
  (params (WeaponType :type E_WeaponType%20Enum :default "NewEnumerator3"))
  (return (Utilities|Select :Index WeaponType :NewEnumerator3 0 :NewEnumerator0 0 :NewEnumerator1 (Variables|WeaponSlots|GetRightHandWeaponSlot) :NewEnumerator2 (Variables|WeaponSlots|GetRightHandWeaponSlot) :NewEnumerator4 (Variables|WeaponSlots|GetLeftHandWeaponSlot))))

(fn GetWeaponSheafeSlot
  (params (WeaponType :type E_WeaponType%20Enum :default "NewEnumerator3"))
  (return (Utilities|Select :Index WeaponType :NewEnumerator3 0 :NewEnumerator0 0 :NewEnumerator1 (Variables|SheathSlots|GetSideArmSheathSlot) :NewEnumerator2 (Variables|SheathSlots|GetBackArmSheathSlot) :NewEnumerator4 (Variables|SheathSlots|GetRangeArmSheathSlot))))

(fn GetAttackRange
  (bind _weaponslot (WeaponSheathing|GetArmedWeaponSlot))
  (bind _baseattackrange (Variables|Default|GetBaseAttackRange))
  (Utilities|IsValid _weaponslot
    (:Is%20Valid
      (bind _range (Class|BPIWeapon|GetRange(Message) (Variables|/Script/Engine.ChildActorComponent|GetChildActor _weaponslot)))
      (return (+ _range _baseattackrange)))
    (:Is%20Not%20Valid
      (return _baseattackrange))))

(fn Init
  (|CallParentFunction)
  (Variables|Components|SetDefaultTurnRate (Variables|/Script/Engine.CharacterMovementComponent|GetRotationRate (Variables|Character|GetCharacterMovement))))

(fn HandleHitDetect
  (|CallParentFunction)
  (bind _drawnweapon (CallFunction|GetDrawnWeapon))
  (Utilities|IsValid _drawnweapon
    (:Is%20Valid
      (bind (_hit _ishit) (Class|BPIWeapon|HitDetect(Message) _drawnweapon))
      (if _ishit
        (if (not (== (.hitactor _hit) self))
          (bind _damageinfo (Class|BPIWeapon|GetDamageInfo(Message) _drawnweapon))
          (Class|PBIDamageable|TakeDamage(Message) (.hitactor _hit) (Utilities|Struct|MakeS_DamageInfo (.basedamage _damageinfo) (.impactpoint _hit) self)))))))

(fn ShootProjectile
  (AttackSystem|RemoveArrow)
  (bind (_isdrawn _drawnweapon) (CallFunction|GetDrawnWeapon))
  (if _isdrawn
    (Class|BPIRangedWeapon|ShootProjectile(Message) _drawnweapon self (Variables|WeaponData|GetBowArrowClass))
    (return true)
    (else
      (return false))))

(fn CheckCanAttackBase
  (bind _canattack (|CallParentFunction))
  (if _canattack
    (return (not (Variables|/Game/TutorialStuff/Components/Sheathing/BPC_SheathingComponent.BPC_SheathingComponent_C|GetIsChangingWeapon (Variables|Default|GetSheathingComponent))))
    (else
      (return false))))

(fn PlayDamageReaction
  (params (S_DamageInfo :type S%20Damage%20Info%20Structure%20%28by%20ref%29))
  (|CallParentFunction S_DamageInfo)
  (Default|ReacttoDamage (Variables|Default|GetProceduralHitReaction) S_DamageInfo)
  (return))

(fn Die
  (params (Damage :type S%20Damage%20Info%20Structure))
  (Utilities|FlowControl|Sequence
    (:then_0
      ;[0.15 0.15 0.15 0.5] stop crazy flight on death
      (Class|PrimitiveComponent|SetAllPhysicsLinearVelocity (Variables|Character|GetMesh) (/ (Transformation|GetVelocity) 4) false))
    (:then_1
      (Default|ReacttoDamage (Variables|Default|GetProceduralHitReaction) Damage)
      (|CallParentFunction Damage))
    (:then_2
      (for _array_element (Utilities|Array|MakeArray (Variables|Default|GetArrowSlot) (Variables|WeaponSlots|GetRightHandWeaponSlot) (Variables|WeaponSlots|GetLeftHandWeaponSlot))
        (CallFunction|DropWeapon _array_element)))))

(fn CheckUseSenseSocket
  ;[0.15 0.15 0.15 0.5] HACK: ue sets a weird Z coord for idle posisition without target. since weapon has aim offset, we prevent using socket so NPCs don't look like fetanol junkies
  (bind _isdrawn (CallFunction|GetDrawnWeapon))
  (if _isdrawn
    (return false)
    (else
      (bind _shoulduse (|CallParentFunction))
      (return _shoulduse))))

(fn RemoveArrow
  (ChildActorComponent|SetChildActorClass (Variables|Default|GetArrowSlot) 0))

(fn HandleAttackEnd
  (Utilities|FlowControl|Sequence
    (:then_0
      (Variables|/Script/Engine.CharacterMovementComponent|SetRotationRate (Variables|Character|GetCharacterMovement) (Variables|Components|GetDefaultTurnRate)))
    (:then_1
      (bind _drawnweapon (CallFunction|GetDrawnWeapon))
      (Class|BPIWeapon|ResetAttack(Message) _drawnweapon))
    (:then_2
      (AttackSystem|RemoveArrow))))

(fn DropWeapon
  (params (Slot :type Child%20Actor%20Component%20Object%20Reference))
  (Utilities|IsValid (Variables|/Script/Engine.ChildActorComponent|GetChildActor Slot)
    (:Is%20Valid
      (Utilities|FlowControl|Sequence
        (:then_0
          (bind _returnvalue (Game|SpawnActorfromClass (Variables|/Script/Engine.ChildActorComponent|GetChildActorClass Slot) (Transformation|GetWorldTransform Slot) "AdjustIfPossibleButAlwaysSpawn" "MultiplyWithRoot" 0 0))
          (Class|BPIDropableItem|DropItem(Message) _returnvalue))
        (:then_1
          (ChildActorComponent|SetChildActorClass Slot 0))
        (:then_2
          (Utilities|Array|Clear (Variables|/Game/TutorialStuff/Components/AttackSystem/BPC_AttackSystem.BPC_AttackSystem_C|GetAttacks (Variables|Default|GetAttackSystem))))))))

(fn ApplyWeapon
  (params (WeaponInfo :type S%20Armed%20Weapon%20Info%20Structure) (WeaponActor :type Actor%20Object%20Reference))
  (bind _attacksystem (Variables|Default|GetAttackSystem))
  (Variables|/Game/TutorialStuff/Components/AttackSystem/BPC_AttackSystem.BPC_AttackSystem_C|SetAttacks _attacksystem (.attacks WeaponInfo))
  (Default|ResetAttackState _attacksystem)
  (Variables|Default|SetBaseAttackRange (.baseattackrange WeaponInfo))
  (bind _damageinfo (Class|BPIWeapon|GetDamageInfo(Message) WeaponActor))
  (Variables|Default|SetAttackStaminaCostValue (.staminacost _damageinfo))
  (bind _animspeedrate (Class|BPIWeapon|GetAnimSpeed(Message) WeaponActor))
  (Variables|/Game/TutorialStuff/Components/AttackSystem/BPC_AttackSystem.BPC_AttackSystem_C|SetAttackSpeedRate (Variables|Default|GetAttackSystem) _animspeedrate)
  (return true))

(fn CheckCanChangeWeapon
  (if (Class|AnimInstance|IsAnyMontagePlaying (Components|SkeletalMesh|GetAnimInstance (Variables|Character|GetMesh)))
    (return false)
    (else
      (bind _isattacking (CallFunction|GetIsAttacking))
      (if _isattacking
        (return false)
        (else
          (return (AI|Components|NavMovement|IsMovingonGround (Variables|Character|GetCharacterMovement))))))))

(fn DrawWeapon
  (params (WeaponType :type E_WeaponType%20Enum :default "NewEnumerator3"))
  (bind _isdrawn (CallFunction|GetDrawnWeapon))
  (if _isdrawn
    (Variables|Default|SetDrawWeaponScheduled WeaponType)
    (bind _isstarted (CallFunction|SheatheWeapon))
    (if _isstarted
      (return true)
      (else
        (Variables|Default|SetDrawWeaponScheduled "NewEnumerator3")
        (return false)))
    (else
      (Variables|Default|SetDrawWeaponScheduled "NewEnumerator3")
      (bind _isstarted_2 (Default|DrawWeapon (Variables|Default|GetSheathingComponent) (Utilities|Select :Index WeaponType :NewEnumerator3 "" :NewEnumerator0 "" :NewEnumerator1 (Variables|WeaponData|GetSwordMoveset) :NewEnumerator2 (Variables|WeaponData|GetSpearMoveset) :NewEnumerator4 (Variables|WeaponData|GetBowMoveset)) (WeaponSheathing|GetWeaponArmSlot WeaponType) (WeaponSheathing|GetWeaponSheafeSlot WeaponType)))
      (return _isstarted_2))))

(fn GetAimPitchYaw
  (bind _returnvalue (Pawn|GetBaseAimRotation))
  (bind _returnvalue_2 (Transformation|GetActorTransform))
  (bind _returnvalue_3 (Math|Rotator|Delta(Rotator) _returnvalue (.rotation _returnvalue_2)))
  (bind _pitchoffset (Class|BPIAttacking|GetAimingPitchOffset(Message) self))
  (return (* (/ (+ _pitchoffset (.pitch _returnvalue_3)) 9e+01) 8e+01) (.yaw _returnvalue_3)))

(fn GetAvailableWeapons
  (for _array_element (Utilities|Array|MakeArray (Variables|SheathSlots|GetRangeArmSheathSlot) (Variables|SheathSlots|GetBackArmSheathSlot) (Variables|SheathSlots|GetSideArmSheathSlot) (Variables|WeaponSlots|GetRightHandWeaponSlot) (Variables|WeaponSlots|GetLeftHandWeaponSlot))
    (Utilities|IsValid _array_element
      (:Is%20Valid
        (Utilities|IsValid (Variables|/Script/Engine.ChildActorComponent|GetChildActor _array_element)
          (:Is%20Valid
            (bind _type (Class|BPIWeapon|GetWeaponType(Message) (Variables|/Script/Engine.ChildActorComponent|GetChildActor _array_element)))
            (if (Utilities|Enum|NotEqual(Enum) _type "NewEnumerator3")
              (Utilities|Array|Add (LocalVariables|GetValidWeapons) (Variables|/Script/Engine.ChildActorComponent|GetChildActor _array_element))))))))
  (return (LocalVariables|GetValidWeapons)))

(fn GetBaseWeaponRange
  (params (Weapon :type Actor%20Object%20Reference))
  (bind _type (Class|BPIWeapon|GetWeaponType(Message) Weapon))
  (return (Utilities|Select :Index _type :NewEnumerator3 0.0 :NewEnumerator0 0.0 :NewEnumerator1 (.baseattackrange (Variables|WeaponData|GetSwordMoveset)) :NewEnumerator2 (.baseattackrange (Variables|WeaponData|GetSpearMoveset)) :NewEnumerator4 (.baseattackrange (Variables|WeaponData|GetBowMoveset)))))

(fn GetDrawnWeapon
  (bind _weaponslot (WeaponSheathing|GetArmedWeaponSlot))
  (bind _childactor (Variables|/Script/Engine.ChildActorComponent|GetChildActor _weaponslot))
  (Utilities|IsValid _weaponslot
    (:Is%20Valid
      (bind _type (Class|BPIWeapon|GetWeaponType(Message) _childactor))
      (return (Utilities|Enum|NotEqual(Enum) _type "NewEnumerator3") _childactor))
    (:Is%20Not%20Valid
      (return false 0))))

(fn GetSheathingComponent
  (return (Variables|Default|GetSheathingComponent)))

(fn SheatheWeapon
  (bind (_isdrawn _drawnweapon) (CallFunction|GetDrawnWeapon))
  (if _isdrawn
    (bind _type (Class|BPIWeapon|GetWeaponType(Message) _drawnweapon))
    (LocalVariables|SetWeaponType _type)
    (bind _isstarted (Default|SheatheWeapon (Variables|Default|GetSheathingComponent) (Utilities|Select :Index (LocalVariables|GetWeaponType) :NewEnumerator3 "" :NewEnumerator0 "" :NewEnumerator1 (Variables|WeaponData|GetSwordMoveset) :NewEnumerator2 (Variables|WeaponData|GetSpearMoveset) :NewEnumerator4 (Variables|WeaponData|GetBowMoveset)) (WeaponSheathing|GetWeaponSheafeSlot (LocalVariables|GetWeaponType)) (WeaponSheathing|GetWeaponArmSlot (LocalVariables|GetWeaponType)) false))
    (return _isstarted)
    (else
      (return false))))