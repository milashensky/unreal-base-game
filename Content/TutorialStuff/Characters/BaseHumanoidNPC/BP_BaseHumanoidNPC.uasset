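; Base humanoid NPC Blueprint that adds an overhead health and stamina widget and predictive aiming at its locked target during attacks.
; While an attack runs, a repeating timer requests AI pawn predictions, with lead time from target distance and a ranged or melee attack speed.
; Successful predictions briefly lock the target component onto the predicted location.
; Health and stamina changes update the widget bars, and death destroys the widget.
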(event OnAttackStart(AttackSystem)
  (params (Attack :type S%20Attack%20Info%20Structure))
  (Variables|Perception|SetIsRequestPrediction true)
  (CallFunction|RequestPredictionTick))

(event OnAttackEnd(AttackSystem)
  (Variables|Perception|SetIsRequestPrediction false))

(event Custom|RequestPredictionTick
  (if (Variables|Perception|GetIsRequestPrediction)
    (AttackPrediction|RequestPrediction)
    (Utilities|FlowControl|Delay 0.2)
    (CallFunction|RequestPredictionTick)))

(event EventHandlePredictionEvent
  (params (Prediction :type AI%20Stimulus%20Structure))
  (if (.bsuccessfullysensed Prediction)
    (Default|LocktoPredictionLocation (Variables|Default|GetTargetLockComponent) (.stimuluslocation Prediction) 0.3)))

(event Collision|EventActorBeginOverlap
  (params (OtherActor :type Actor%20Object%20Reference)))

(fn ConstructionScript
  (|CallParentFunction))

(fn BuildUI
  (bind _health (CallFunction|GetCurrentHealth))
  (CallFunction|SetHealthWidgetValue _health)
  (bind _currentstamina (CallFunction|GetCurrentStamina))
  (CallFunction|SetStaminaWidgetValue _currentstamina))

(fn SetHealthWidgetValue
  (params (Health :type Integer))
  (bind _healthbarwidget (Variables|Default|GetHealthBarWidget))
  (|CallParentFunction Health)
  (bind _maxhealth (CallFunction|GetMaxHealth))
  (Utilities|IsValid _healthbarwidget
    (:Is%20Valid
      (bind _aswb_npc_widget (Utilities|Casting|CastToWB_NpcWidget (UserInterface|GetWidget _healthbarwidget)))
      (Progress|SetPercent (Variables|/Game/TutorialStuff/UI/Widgets/WB_NpcWidget.WB_NpcWidget_C|GetHealthBar _aswb_npc_widget) (/ (Math|Conversions|ToFloat(Integer) Health) (Math|Conversions|ToFloat(Integer) (Math|Integer|Clamp(Integer) _maxhealth 1 _maxhealth)))))))

(fn SetStaminaWidgetValue
  (params (Stamina :type Integer))
  (bind _healthbarwidget (Variables|Default|GetHealthBarWidget))
  (|CallParentFunction Stamina)
  (bind _maxstamina (CallFunction|GetMaxStamina))
  (Utilities|IsValid _healthbarwidget
    (:Is%20Valid
      (bind _aswb_npc_widget (Utilities|Casting|CastToWB_NpcWidget (UserInterface|GetWidget _healthbarwidget)))
      (Progress|SetPercent (Variables|/Game/TutorialStuff/UI/Widgets/WB_NpcWidget.WB_NpcWidget_C|GetStaminaBar _aswb_npc_widget) (/ (Math|Conversions|ToFloat(Integer) Stamina) (Math|Conversions|ToFloat(Integer) (Math|Integer|Clamp(Integer) _maxstamina 1 _maxstamina)))))))

(fn Die
  (params (Damage :type S%20Damage%20Info%20Structure))
  (|CallParentFunction Damage)
  (Components|DestroyComponent (Variables|Default|GetHealthBarWidget)))

(fn RequestPrediction
  (bind _targetlockcomponent (Variables|Default|GetTargetLockComponent))
  (bind _locktarget (Variables|/Game/TutorialStuff/Components/TargetLockComponent/BPC_TargetLockComponent.BPC_TargetLockComponent_C|GetLockTarget _targetlockcomponent))
  (bind _output_get (LocalVariables|SetLocked%20Target _locktarget))
  (Utilities|IsValid _output_get
    (:Is%20Valid
      (LocalVariables|SetDistanceToTarget (Transformation|GetDistanceTo self _locktarget))
      (Utilities|FlowControl|Sequence
        (:then_0
          (bind (_isdrawn _drawnweapon) (CallFunction|GetDrawnWeapon))
          (if _isdrawn
            (bind _isranged (Class|BPIRangedWeapon|GetIsRanged(Message) _drawnweapon))
            (if _isranged
              ;[0.15 0.15 0.15 0.5] TODO: consider dynamic value
              (LocalVariables|SetAttackSpeed 1.9e+03)
              (else
                (LocalVariables|SetAttackSpeed 6e+02)))))
        (:then_1
          (if (> (LocalVariables|GetAttackSpeed) 0.0)
            (Class|AISensePrediction|RequestPawnPredictionEvent self (LocalVariables|GetLocked%20Target) (/ (LocalVariables|GetDistanceToTarget) (LocalVariables|GetAttackSpeed)))))))))

(fn Init
  (|CallParentFunction)
  (UI|BuildUI))

(fn GetAimingPitchOffset
  (bind _attacksystem (Variables|Default|GetAttackSystem))
  (Utilities|IsValid _attacksystem
    (:Is%20Valid
      (if (Variables|/Game/TutorialStuff/Components/AttackSystem/BPC_AttackSystem.BPC_AttackSystem_C|GetIsAttacking _attacksystem)
        (return 15.0)
        (else
          (return 2e+01))))
    (:Is%20Not%20Valid
      (return 0.0))))