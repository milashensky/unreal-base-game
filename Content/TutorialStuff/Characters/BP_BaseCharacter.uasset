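; Base character Blueprint providing shared combat, movement and stat logic, with empty or default functions such as Init, HandleHitDetect and widget setters.
; Delegates to health, stamina, attack, movement and target-lock components, exposed through getters and wrappers.
; Stamina gates jumps, attacks and sprinting, with sprint drain polled by a retriggerable-delay loop.
; An attack token queue coordinates AI attackers, and death disables movement and attacks, then ragdolls the mesh.
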(event OnDamageTaken(HealthComponent)
  (params (Damage :type S%20Damage%20Info%20Structure))
  (Health|PlayDamageReaction Damage))

(event OnSpintStart(SprintWalkRunMovement)
  ;[0.15 0.15 0.15 0.5] Sprinting
  (CallFunction|SprintTick))

(event OnSpintEnd(SprintWalkRunMovement)
  ;[0.15 0.15 0.15 0.5] Sprinting
  (CallFunction|SprintTick)
  (Default|StartPassiveStaminaRestore (Variables|Default|GetStaminaComponent)))

(event OnOutOfStamina(StaminaComponent)
  ;[0.15 0.15 0.15 0.5] Sprinting
  (CallFunction|StartRun))

(event OnHealthChange(HealthComponent)
  (params (New%20Health :type Integer))
  ;[0.15 0.15 0.15 0.5] StatsUI
  (UI|SetHealthWidgetValue New%20Health))

(event OnStaminaChange(StaminaComponent)
  (params (New%20Stamina :type Integer))
  ;[0.15 0.15 0.15 0.5] StatsUI
  (UI|SetStaminaWidgetValue New%20Stamina))

(event OnDeath(HealthComponent)
  (params (Damage :type S%20Damage%20Info%20Structure))
  ;[0.15 0.15 0.15 0.5] Death ragdoll
  (Health|Die Damage)
  (Utilities|FlowControl|Delay 2.0))

(event Custom|SprintTick
  ;[0.15 0.15 0.15 0.5] Sprinting
  (bind _isdead (CallFunction|GetIsDead))
  (if (not _isdead)
    (Movement|HandleSprintDrain)
    (Utilities|FlowControl|RetriggerableDelay 0.2)
    (CallFunction|SprintTick)))

(event EventSetLockIndicatorDisplay
  (params (IsVisible :type Boolean))
  ;[0.15 0.15 0.15 0.5] TargetLock
  (Rendering|SetVisibility (Variables|Default|GetTargetLockIndicator) IsVisible false))

(event EventHitDetect
  ;[0.15 0.15 0.15 0.5] AttackComponent
  (bind _isdead (CallFunction|GetIsDead))
  (if (not _isdead)
    (AttackSystem|HandleHitDetect)))

(event EventOnLanded
  (params (Hit :type Hit%20Result%20Structure%20%28by%20ref%29))
  ;[0.15 0.15 0.15 0.5] Jumping
  (Default|StartPassiveStaminaRestore (Variables|Default|GetStaminaComponent))
  (Class|Actor|MakeNoise 1.0 self (Transformation|GetActorLocation) 0.0 "None"))

(event EventRemoveTargetLock
  ;[0.15 0.15 0.15 0.5] TargetLock
  (Default|EndTargetLock (Variables|Default|GetTargetLockComponent))
  (Variables|Default|SetUseSenseSocket true))

(event EventBeginPlay
  ;[0.15 0.15 0.15 0.5] Start Init
  (Init|Init))

(event EventReturnToken
  (params (Attacking%20Actor :type Actor%20Object%20Reference))
  ;[0.15 0.15 0.15 0.5] AI attack coordination
  (Default|ReturnToken (Variables|Default|GetAttackTokenQueue) Attacking%20Actor))

(event EventEndHitDetect
  ;[0.15 0.15 0.15 0.5] AttackComponent
)

(event EventStartHitDetect
  ;[0.15 0.15 0.15 0.5] AttackComponent
)

(event EventResetAttackState
  ;[0.15 0.15 0.15 0.5] AttackComponent
  (Default|ResetAttackState (Variables|Default|GetAttackSystem)))

(event EventStartWalk
  ;[0.15 0.15 0.15 0.5] Movement
  (Default|StartWalk (Variables|Default|GetSprintWalkRunMovement)))

(event EventOnJumped
  ;[0.15 0.15 0.15 0.5] Jumping
  (Default|DrainStamina (Variables|Default|GetStaminaComponent) (Variables|Default|GetJumpStaminaCostValue) false))

(event EventStartRun
  ;[0.15 0.15 0.15 0.5] Movement
  (Default|StartRun (Variables|Default|GetSprintWalkRunMovement)))

(event EventStartSprint
  ;[0.15 0.15 0.15 0.5] Sprinting
  (Default|StartSprint (Variables|Default|GetSprintWalkRunMovement)))

(event EventLockTarget
  (params (LockTarget :type Actor%20Object%20Reference))
  ;[0.15 0.15 0.15 0.5] TargetLock
  (Default|SetTargetLockActor (Variables|Default|GetTargetLockComponent) LockTarget)
  (Variables|Default|SetUseSenseSocket false))

(fn ConstructionScript)

(fn Die
  (params (NewParam :type S%20Damage%20Info%20Structure))
  (bind _mesh (Variables|Character|GetMesh))
  (CallFunction|RemoveTargetLock)
  (Pawn|Components|CharacterMovement|SetMovementMode (Variables|Character|GetCharacterMovement) "MOVE_Walking" 0)
  (Pawn|Components|CharacterMovement|DisableMovement (Variables|Character|GetCharacterMovement))
  (Collision|SetActorEnableCollision true)
  (Physics|SetSimulatePhysics _mesh true)
  (Collision|SetCollisionEnabled _mesh "QueryAndPhysics")
  (Collision|SetCollisionEnabled (Variables|Default|GetCapsuleComponent) "NoCollision")
  (Components|Activation|Deactivate (Variables|Default|GetAttackSystem))
  (Audio|PlaySoundatLocation (Variables|Default|GetDeathSound) (Transformation|GetActorLocation) "0, 0, 0" 1.0 1.0 0.0 0 0 self 0))

(fn SetHealthWidgetValue
  (params (Health :type Integer)))

(fn SetStaminaWidgetValue
  (params (Stamina :type Integer)))

(fn Init)

(fn CanJumpInternal
  (if (AI|Components|NavMovement|IsMovingonGround (Variables|Character|GetCharacterMovement))
    (bind _canperform (Default|GetHasEnoughStaminaforAction (Variables|Default|GetStaminaComponent) (Variables|Default|GetJumpStaminaCostValue)))
    (return _canperform)
    (else
      (return false))))

(fn HandleHitDetect)

(fn HandleSprintDrain
  (if (and (> (Math|Vector|VectorLength (Transformation|GetVelocity)) 7e+01) (Components|ComponentHasTag (Variables|Default|GetSprintWalkRunMovement) "IsSprinting"))
    (bind _cansprint (CallFunction|CheckCanSprint))
    (if _cansprint
      (Default|StartStaminaDrain (Variables|Default|GetStaminaComponent) (Variables|Default|GetSprintStaminaCostPerSec))
      (else
        (Default|StopStaminaDrain (Variables|Default|GetStaminaComponent))))
    (elif (Variables|/Game/TutorialStuff/Components/Stamina/BPC_StaminaComponent.BPC_StaminaComponent_C|GetIsStaminaDraining (Variables|Default|GetStaminaComponent))
      (Default|StartPassiveStaminaRestore (Variables|Default|GetStaminaComponent)))))

(fn CheckCanAttackBase
  (if (AI|Components|NavMovement|IsMovingonGround (Variables|Character|GetCharacterMovement))
    (bind _canperform (Default|GetHasEnoughStaminaforAction (Variables|Default|GetStaminaComponent) (Variables|Default|GetAttackStaminaCostValue)))
    (if _canperform
      (return (Components|Activation|IsActive (Variables|Default|GetAttackSystem)))
      (else
        (return false)))
    (else
      (return false))))

(fn PlayDamageReaction
  (params (S_DamageInfo :type S%20Damage%20Info%20Structure%20%28by%20ref%29))
  (Audio|PlaySoundatLocation (Variables|Default|GetHitSound) (Transformation|GetActorLocation) "0, 0, 0" 1.0 1.0 0.0 0 0 self 0))

(fn Attack
  (bind _canattack (CallFunction|CheckCanAttack))
  (if _canattack
    ;[0.15 0.15 0.15 0.5] TODO: crouch attack?
    (Character|UnCrouch)
    (bind _isattacked (Default|Attack (Variables|Default|GetAttackSystem)))
    (if _isattacked
      (Default|DrainStamina (Variables|Default|GetStaminaComponent) (Variables|Default|GetAttackStaminaCostValue) true)
      (return true)
      (else
        (return false)))
    (else
      (return false))))

(fn CheckCanAttack
  (bind _canattack (AttackSystem|CheckCanAttackBase))
  (return _canattack))

(fn CheckCanbeAttacked
  (params (Attacking%20Actor :type Actor%20Object%20Reference) (Bucket :type E_AttackTokenBuckets%20Enum :default "NewEnumerator0"))
  (bind _result (Default|CheckCanbeAttacked (Variables|Default|GetAttackTokenQueue) Attacking%20Actor Bucket))
  (return _result))

(fn CheckCanSprint
  (bind _isattacking (CallFunction|GetIsAttacking))
  (if (and (not _isattacking) (AI|Components|NavMovement|IsMovingonGround (Variables|Character|GetCharacterMovement)))
    (bind _canperform (Default|GetHasEnoughStaminaforAction (Variables|Default|GetStaminaComponent) (Variables|Default|GetSprintStaminaCostPerSec)))
    (return _canperform)
    (else
      (return false))))

(fn GetAimingPitchOffset
  (return 0.0))

(fn GetAttackComponent
  (return (Variables|Default|GetAttackSystem)))

(fn GetAttackRange
  (return (Variables|Default|GetBaseAttackRange)))

(fn GetCharacterMovementComponent
  (return (Variables|Character|GetCharacterMovement)))

(fn GetCurrentHealth
  (return (Variables|/Game/TutorialStuff/Components/Health/BPC_HealthComponent.BPC_HealthComponent_C|GetCurrentHealth (Variables|Default|GetHealthComponent))))

(fn GetCurrentStamina
  (return (Variables|/Game/TutorialStuff/Components/Stamina/BPC_StaminaComponent.BPC_StaminaComponent_C|GetCurrentStamina (Variables|Default|GetStaminaComponent))))

(fn GetHealthComponent
  (return (Variables|Default|GetHealthComponent)))

(fn GetIsAttacking
  (return (Variables|/Game/TutorialStuff/Components/AttackSystem/BPC_AttackSystem.BPC_AttackSystem_C|GetIsAttacking (Variables|Default|GetAttackSystem))))

(fn GetIsDead
  (return (Variables|/Game/TutorialStuff/Components/Health/BPC_HealthComponent.BPC_HealthComponent_C|GetIsDead (Variables|Default|GetHealthComponent))))

(fn GetLockedLocation
  (bind (_islocked _locktarget _location) (Default|GetTargetLockLocation (Variables|Default|GetTargetLockComponent)))
  (return _islocked _location _locktarget))

(fn GetMaxHealth
  (return (Variables|/Game/TutorialStuff/Components/Health/BPC_HealthComponent.BPC_HealthComponent_C|GetMaxHealth (Variables|Default|GetHealthComponent))))

(fn GetMaxStamina
  (return (Variables|/Game/TutorialStuff/Components/Stamina/BPC_StaminaComponent.BPC_StaminaComponent_C|GetMaxStamina (Variables|Default|GetStaminaComponent))))

(fn GetSkeletalMeshComponent
  (return (Variables|Character|GetMesh)))

(fn GetTargetLockPosition
  (return (not (Variables|/Game/TutorialStuff/Components/Health/BPC_HealthComponent.BPC_HealthComponent_C|GetIsDead (Variables|Default|GetHealthComponent))) (Transformation|GetWorldLocation (Variables|Default|GetTargetLock))))

(fn GetTeamId
  (return (Variables|Default|GetTeamId)))

(fn GetWarpingComponent
  (return (Variables|Default|GetMotionWarping)))

(fn Heal
  (params (Amount :type Integer))
  (bind _newhealth (Default|Heal (Variables|Default|GetHealthComponent) Amount))
  (return _newhealth))

(fn IsDamageable
  (return true))

(fn ShootProjectile
  (return false))

(fn TakeDamage
  (params (Damage :type S%20Damage%20Info%20Structure))
  (bind _wasdamaged (Default|TakeDamage (Variables|Default|GetHealthComponent) Damage))
  (return _wasdamaged))

(fn TakeToken
  (params (Attacking%20Actor :type Actor%20Object%20Reference))
  (bind _result (Default|TakeToken (Variables|Default|GetAttackTokenQueue) Attacking%20Actor))
  (return _result))