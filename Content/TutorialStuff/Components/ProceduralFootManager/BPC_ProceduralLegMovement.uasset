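; Actor component that procedurally steps the legs of its owner's skeletal mesh, exposing per-bone foot transforms with curve-driven step height.
; Each tick it picks a gait by speed, blends its parameters and advances a speed-scaled global cycle timer.
; Legs start steps at their cycle offsets, sphere-tracing targets along velocity and interpolating toward them by curve.
; Running steps are rescaled and redirected as step length or direction changes, then re-traced to ground.
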(event EventBeginPlay
  (Variables|State|SetIsReady false)
  (bind _skeletalmeshcomponent (Class|BPIwithSkeletalMeshComponent|GetSkeletalMeshComponent(Message) (Components|GetOwner)))
  (Utilities|IsValid _skeletalmeshcomponent
    (:Is%20Valid
      (Variables|Default|SetSkeletal%20Mesh%20Component _skeletalmeshcomponent)
      (Init|InitGait)
      (Init|InitLegs)
      (Variables|State|SetIsReady true))))

(event EventTick
  (params (DeltaSeconds :type Float%20%28single-precision%29))
  (if (Variables|State|GetIsReady)
    (Variables|Private/Global|SetDeltaTime DeltaSeconds)
    (Calculation/Global|CalculateVelocity)
    (Calculation/Global|SelectGait)
    (Calculation/Global|RunGlobalTimer)
    (Calculation/Global|UpdateLegsPlacement)))

(fn GetLegTransform
  (params (BoneName :type Name))
  (bind _legstatesbybone (Variables|Private/Step|GetLegStatesByBone))
  (bind _value (Utilities|Map|Find _legstatesbybone BoneName))
  (bind _output_get (LocalVariables|SetLegTransform (.WorldTransform (Utilities|Struct|BreakS_BoneLocation (.interpolatedlocation _value)))))
  (return (Math|Transform|MakeTransform (+ (.Location (Math|Transform|BreakTransform _output_get)) (Math|Vector|MakeVector 0.0 0.0 (* (Class|KismetMathLibrary|GetRuntimeFloatCurveValue (Variables|Config|GetStepHeightCurve) (.progress _value) 0.0) (Variables|Private/Step|GetStepHeight)))) (.rotation (LocalVariables|GetLegTransform)) (.scale (LocalVariables|GetLegTransform)))))

(fn FindMatchingGait
  (LocalVariables|SetCurrentSpeed (Math|Vector|VectorLength (Variables|Private/Global|GetVelocity)))
  (for _array_element (Variables|Config|GetGaits)
    (if (and (<= (.MinSpeed (Utilities|Struct|BreakS_GaitInfo _array_element)) (LocalVariables|GetCurrentSpeed)) (>= (.MinSpeed (Utilities|Struct|BreakS_GaitInfo _array_element)) (.minspeed (LocalVariables|GetSelectedGait))))
      (LocalVariables|SetSelectedGait _array_element)))
  (return (LocalVariables|GetSelectedGait)))

(fn SelectGait
  (bind _gait (Calculation/Global|FindMatchingGait))
  (Variables|Private/Global|SetActiveGait _gait)
  (Variables|Private/Step|SetCycleDuration (Math|Float|Lerp (Variables|Private/Step|GetCycleDuration) (.CycleDuration (Utilities|Struct|BreakS_GaitInfo (Variables|Private/Global|GetActiveGait))) (Variables|Config|GetBlendFactor)))
  (Variables|Private/Step|SetStepLength (Math|Float|Lerp (Variables|Private/Step|GetStepLength) (.StepLength (Utilities|Struct|BreakS_GaitInfo (Variables|Private/Global|GetActiveGait))) (Variables|Config|GetBlendFactor)))
  (Variables|Private/Step|SetOptimalMovementSpeed (Math|Float|Lerp (Variables|Private/Step|GetOptimalMovementSpeed) (.MovementSpeed (Utilities|Struct|BreakS_GaitInfo (Variables|Private/Global|GetActiveGait))) (Variables|Config|GetBlendFactor)))
  (Variables|Private/Step|SetStepHeight (Math|Float|Lerp (Variables|Private/Step|GetStepHeight) (.StepHeight (Utilities|Struct|BreakS_GaitInfo (Variables|Private/Global|GetActiveGait))) (Variables|Config|GetBlendFactor))))

(fn CalculateVelocity
  (Variables|Private/Global|SetPreviousVelocity (Variables|Private/Global|GetPreviousVelocity))
  (Variables|Private/Global|SetVelocity (Transformation|GetVelocity (Components|GetOwner))))

(fn RunGlobalTimer
  (bind _velocity (Variables|Private/Global|GetVelocity))
  (bind _returnvalue (Math|Vector|VectorLength _velocity))
  (Utilities|FlowControl|Sequence
    (:then_0
      (if (<= _returnvalue 0.001)
        (LocalVariables|SetSpeedMultiplier 1.0)
        (else
          (LocalVariables|SetSpeedMultiplier (/ _returnvalue (Helpers|GetSafeDivider (Variables|Private/Step|GetOptimalMovementSpeed) (Helpers|GetSafeDivider _returnvalue 1.0)))))))
    (:then_1
      (bind _output_get (Variables|Private/Global|SetDeltaProgress (* (/ (Variables|Private/Global|GetDeltaTime) (Variables|Private/Step|GetCycleDuration)) (LocalVariables|GetSpeedMultiplier))))
      (bind _output_get_2 (Variables|Private/Global|SetGlobalCycleProgress (Math|Float|%(Float) (+ _output_get (Variables|Private/Global|GetGlobalCycleProgress)) 1.0)))
      (CallFunction|PrintTextLog (Utilities|Array|MakeArray "timer:" (Utilities|String|ToString(Float) _output_get_2) "current delta:" (Utilities|String|ToString(Float) (Variables|Private/Global|GetDeltaProgress))) "timer" 2.0 "(R=0.000000,G=0.855387,B=1.000000,A=1.000000)"))))

(fn UpdateLegsPlacement
  (bind (_keypin _valuepin) (Utilities|Map|ForEachLoop(Map) (Variables|Private/Step|GetLegStatesByBone))
    (:then
      (bind _updatedlegstate (Calculation/Leg|UpdateLeg _keypin _valuepin))
      (Utilities|Map|Add (Variables|Private/Step|GetLegStatesByBone) _keypin _updatedlegstate))))

(fn InitGait
  (bind _gait (Calculation/Global|FindMatchingGait))
  (bind _output_get (Variables|Private/Global|SetActiveGait _gait))
  (Variables|Private/Step|SetStepLength (.StepLength (Utilities|Struct|BreakS_GaitInfo _output_get)))
  (Variables|Private/Step|SetStepHeight (.StepHeight (Utilities|Struct|BreakS_GaitInfo _output_get)))
  (Variables|Private/Step|SetCycleDuration (.CycleDuration (Utilities|Struct|BreakS_GaitInfo _output_get)))
  (Variables|Private/Step|SetOptimalMovementSpeed (.MovementSpeed (Utilities|Struct|BreakS_GaitInfo _output_get))))

(fn InitLegs
  (bind _keypin (Utilities|Map|ForEachLoop(Map) (.LegByBone (Utilities|Struct|BreakS_GaitInfo (Variables|Private/Global|GetActiveGait))))
    (:then
      (bind _output_get (LocalVariables|SetInteratedBoneName _keypin))
      (Utilities|Map|Add (Variables|Private/Global|GetActorLegInitialLocalTransform) _output_get (Helpers|FromWorld (Transformation|GetBoneTransform (Variables|Default|GetSkeletal%20Mesh%20Component) (LocalVariables|GetInteratedBoneName) "RTS_World")))
      (bind _outtransform (Helpers|TraceLegLocation (LocalVariables|GetInteratedBoneName) "0, 0, 0"))
      (Utilities|Map|Add (Variables|Private/Step|GetLegStatesByBone) (LocalVariables|GetInteratedBoneName) (Utilities|Struct|MakeS_CalculatedLegInfo _outtransform _outtransform (Utilities|Struct|MakeS_BoneLocation (Transformation|GetBoneTransform (Variables|Default|GetSkeletal%20Mesh%20Component) (LocalVariables|GetInteratedBoneName) "RTS_World") (Helpers|FromWorld (Transformation|GetBoneTransform (Variables|Default|GetSkeletal%20Mesh%20Component) (LocalVariables|GetInteratedBoneName) "RTS_World"))) 0.0 0.0 0.0 "0.000000,0.000000,0.000000" 0.0)))))

(fn TraceatLocation
  (params (TargetTransform :type Transform))
  (bind _location (Math|Transform|BreakTransform TargetTransform))
  (bind _traceheight (Variables|Config|GetTraceHeight))
  (bind (_outhit _returnvalue) (Collision|SphereTraceByChannel (+ _location (Math|Vector|MakeVector 0.0 0.0 _traceheight)) (- _location (Math|Vector|MakeVector 0.0 0.0 _traceheight)) (Variables|Config|GetTraceRadius) "TraceTypeQuery1" false 0 "ForOneFrame" true "(R=1.000000,G=0.000000,B=0.000000,A=1.000000)" "(R=0.000000,G=1.000000,B=0.000000,A=1.000000)" 1e+01))
  (if _returnvalue
    (return (Math|Transform|MakeTransform (.impactpoint _outhit) (.rotation TargetTransform) (.scale TargetTransform)))
    (else
      (return TargetTransform))))

(fn TraceLegLocation
  (params (BoneName :type Name) (Target :type Vector))
  (bind _actorleginitiallocaltransform (Variables|Private/Global|GetActorLegInitialLocalTransform))
  (bind (_value _returnvalue) (Utilities|Map|Find _actorleginitiallocaltransform BoneName))
  (LocalVariables|SetLegTransform (Transformation|GetBoneTransform (Variables|Default|GetSkeletal%20Mesh%20Component) BoneName "RTS_World"))
  (Utilities|FlowControl|Sequence
    (:then_0
      (if _returnvalue
        ;[0.15 0.15 0.15 0.5] Get Leg initial transform and then convert it to world space
        (LocalVariables|SetStartLocation (.Location (Math|Transform|BreakTransform (Helpers|ToWorld _value))))
        (else
          (LocalVariables|SetStartLocation (.location (LocalVariables|GetLegTransform))))))
    (:then_1
      (bind _outtransform (Helpers|TraceatLocation (Math|Transform|MakeTransform (+ (LocalVariables|GetStartLocation) Target) (.rotation (LocalVariables|GetLegTransform)) (.scale (LocalVariables|GetLegTransform)))))
      (return _outtransform))))

(fn ToWorld
  (params (Local :type Transform))
  (return (Math|Transform|ComposeTransforms Local (Transformation|GetWorldTransform (Variables|Default|GetSkeletal%20Mesh%20Component)))))

(fn FromWorld
  (params (World :type Transform))
  (return (Math|Transform|ComposeTransforms World (Math|Transform|InvertTransform (Transformation|GetWorldTransform (Variables|Default|GetSkeletal%20Mesh%20Component))))))

(fn GetSafeDivider
  (params (value :type Float%20%28double-precision%29) (fallback :type Float%20%28double-precision%29))
  (if (== value 0.0)
    (return fallback)
    (else
      (return value))))

(fn UpdateLeg
  (params (BoneName :type Name) (LegState :type S%20Calculated%20Leg%20Info%20Structure))
  (bind _steplength (Variables|Private/Step|GetStepLength))
  (Utilities|FlowControl|Sequence
    (:then_0
      (LocalVariables|SetGaitLegConfig (.Value (Utilities|Map|Find (.legbybone (Variables|Private/Global|GetActiveGait)) BoneName)))
      (LocalVariables|SetLerpedPositionOffset (Math|Vector|Lerp(Vector) (.placementoffset LegState) (.PositionOffset (Utilities|Struct|BreakS_GaitLegInfo (LocalVariables|GetGaitLegConfig))) (Variables|Config|GetBlendFactor))))
    (:then_1
      (LocalVariables|SetLerpedOffset (Math|Float|Lerp (.offset LegState) (.CycleOffset (Utilities|Struct|BreakS_GaitLegInfo (LocalVariables|GetGaitLegConfig))) (Variables|Config|GetBlendFactor))))
    (:then_2
      (bind _output_get (LocalVariables|SetStepVector (* (Math|Vector|Normalize (Variables|Private/Global|GetVelocity)) _steplength)))
      ;[0.15 0.15 0.15 0.5] Log
      (CallFunction|PrintTextLog (Utilities|Array|MakeArray (Utilities|String|ToString(Float) (Math|Vector|VectorLength _output_get)) "vector length" (Utilities|String|ToString(Float) _steplength) "step lenth") "speed" 2.0 "(R=0.000000,G=0.855387,B=1.000000,A=1.000000)"))
    (:then_3
      (bind _shouldmove (Calculation/Leg|CheckShouldMove LegState))
      (if _shouldmove
        ;[0.15 0.15 0.15 0.5] Start New step
        (bind _outtransform (Helpers|TraceLegLocation BoneName (LocalVariables|GetStepVector)))
        (LocalVariables|SetUpdatedLeg (Utilities|Struct|MakeS_CalculatedLegInfo (.WorldTransform (Utilities|Struct|BreakS_BoneLocation (.interpolatedlocation LegState))) _outtransform (.interpolatedlocation LegState) (LocalVariables|GetLerpedOffset) 0.0 (.progress LegState) (LocalVariables|GetLerpedPositionOffset) (Variables|Private/Step|GetStepLength)))
        (else
          ;[0.15 0.15 0.15 0.5] Update Running Step
          (bind (_interpolatedstarttransform _interpolatedtargettransform _interpolatedsteplength) (Calculation/Leg|InterpolateLegTarget LegState BoneName))
          (LocalVariables|SetUpdatedLeg (Utilities|Struct|MakeS_CalculatedLegInfo _interpolatedstarttransform _interpolatedtargettransform (.interpolatedlocation LegState) (LocalVariables|GetLerpedOffset) (+ (.progress LegState) (Variables|Private/Global|GetDeltaProgress)) (.progress LegState) (LocalVariables|GetLerpedPositionOffset) _interpolatedsteplength)))))
    (:then_4
      ;[0.15 0.15 0.15 0.5] Log
      (CallFunction|PrintTextLog (Utilities|Array|MakeArray (Utilities|String|ToString(Name) BoneName) "leg" (Utilities|String|ToString(Float) (Class|KismetMathLibrary|GetRuntimeFloatCurveValue (.lengthcurve (LocalVariables|GetGaitLegConfig)) (Math|Float|Clamp(Float) (.progress (LocalVariables|GetUpdatedLeg))) 0.0)) "alpha" (Utilities|String|ToString(Float) (.steplength (LocalVariables|GetUpdatedLeg))) "step length," (Utilities|String|ToString(Float) (.offset (LocalVariables|GetUpdatedLeg))) "offset," (Utilities|String|ToString(Float) (.CycleOffset (Utilities|Struct|BreakS_GaitLegInfo (LocalVariables|GetGaitLegConfig)))) "target offset") BoneName 2.0 "(R=0.000000,G=0.855387,B=1.000000,A=1.000000)")
      ;[0.15 0.15 0.15 0.5] Interpolate Running Step
      (return (Utilities|Struct|MakeS_CalculatedLegInfo (.lockedworldtransform (LocalVariables|GetUpdatedLeg)) (.targetworldtransform (LocalVariables|GetUpdatedLeg)) (Utilities|Struct|MakeS_BoneLocation (Math|Transform|Lerp(Transform) (.lockedworldtransform (LocalVariables|GetUpdatedLeg)) (.targetworldtransform (LocalVariables|GetUpdatedLeg)) (Class|KismetMathLibrary|GetRuntimeFloatCurveValue (.lengthcurve (LocalVariables|GetGaitLegConfig)) (Math|Float|Clamp(Float) (.progress (LocalVariables|GetUpdatedLeg))) 0.0)) (Helpers|FromWorld (Math|Transform|Lerp(Transform) (.lockedworldtransform (LocalVariables|GetUpdatedLeg)) (.targetworldtransform (LocalVariables|GetUpdatedLeg)) (Class|KismetMathLibrary|GetRuntimeFloatCurveValue (.lengthcurve (LocalVariables|GetGaitLegConfig)) (Math|Float|Clamp(Float) (.progress (LocalVariables|GetUpdatedLeg))) 0.0)))) (.offset (LocalVariables|GetUpdatedLeg)) (.progress (LocalVariables|GetUpdatedLeg)) (.previousprogress (LocalVariables|GetUpdatedLeg)) (.placementoffset (LocalVariables|GetUpdatedLeg)) (.steplength (LocalVariables|GetUpdatedLeg)))))))

(fn CheckShouldMove
  (params (Leg :type S%20Calculated%20Leg%20Info%20Structure))
  (bind _returnvalue (- (.progress Leg) (.previousprogress Leg)))
  (LocalVariables|SetLeg%20Offset (.offset Leg))
  (Utilities|FlowControl|Sequence
    (:then_0
      (if (>= (.progress Leg) 1.0)
        (return true)))
    (:then_1
      (if (< _returnvalue 0.0)
        (LocalVariables|SetLegProgressDelta (+ _returnvalue 1.0))
        (else
          (LocalVariables|SetLegProgressDelta _returnvalue))))
    (:then_2
      (LocalVariables|SetPreviousProgress (- (Variables|Private/Global|GetGlobalCycleProgress) (LocalVariables|GetLegProgressDelta))))
    (:then_3
      (return (or (and (<= (LocalVariables|GetPreviousProgress) (LocalVariables|GetLeg%20Offset)) (>= (Variables|Private/Global|GetGlobalCycleProgress) (LocalVariables|GetLeg%20Offset))) (and (<= (+ (LocalVariables|GetPreviousProgress) 1.0) (LocalVariables|GetLeg%20Offset)) (>= (+ (Variables|Private/Global|GetGlobalCycleProgress) 1.0) (LocalVariables|GetLeg%20Offset))))))))

(fn RemapStepLength
  (params (Leg :type S%20Calculated%20Leg%20Info%20Structure) (StepLength :type Float%20%28double-precision%29))
  (bind (_lockedworldtransform _targetworldtransform _interpolatedlocation) (Utilities|Struct|BreakS_CalculatedLegInfo Leg))
  (bind (_lockedworldtransform_2 _targetworldtransform_2 _interpolatedlocation_2 _offset _progress _previousprogress _placementoffset _steplength) (Utilities|Struct|BreakS_CalculatedLegInfo Leg))
  (LocalVariables|SetLockedPosition _lockedworldtransform)
  (LocalVariables|SetTargetPosition _targetworldtransform)
  (Utilities|FlowControl|Sequence
    (:then_0
      (if (< (Math|Vector|Distance(Vector) (.Location (Math|Transform|BreakTransform _lockedworldtransform_2)) (.Location (Math|Transform|BreakTransform _targetworldtransform_2))) 5.0)
        (return (Utilities|Struct|MakeS_CalculatedLegInfo (LocalVariables|GetLockedPosition) (LocalVariables|GetTargetPosition) (.interpolatedlocation Leg) (.offset Leg) (.progress Leg) (.previousprogress Leg) (.placementoffset Leg) (.steplength Leg)) false)))
    (:then_1
      (if (or (< _steplength 0.0001) (< (CallFunction|Diff _steplength StepLength) 1.0))
        (return (Utilities|Struct|MakeS_CalculatedLegInfo (LocalVariables|GetLockedPosition) (LocalVariables|GetTargetPosition) (.interpolatedlocation Leg) (.offset Leg) (.progress Leg) (.previousprogress Leg) (.placementoffset Leg) (.steplength Leg)) false)
        (else
          (LocalVariables|SetScaleFactor (/ StepLength (.StepLength (Utilities|Struct|BreakS_CalculatedLegInfo Leg)))))))
    (:then_2
      (LocalVariables|SetCurrentLocation (.Location (Math|Transform|BreakTransform (.WorldTransform (Utilities|Struct|BreakS_BoneLocation _interpolatedlocation))))))
    (:then_3
      (return (Utilities|Struct|MakeS_CalculatedLegInfo (Math|Transform|MakeTransform (- (LocalVariables|GetCurrentLocation) (* (- (LocalVariables|GetCurrentLocation) (.Location (Math|Transform|BreakTransform (LocalVariables|GetLockedPosition)))) (LocalVariables|GetScaleFactor))) (.rotation (LocalVariables|GetLockedPosition)) (.scale (LocalVariables|GetLockedPosition))) (Math|Transform|MakeTransform (+ (LocalVariables|GetCurrentLocation) (* (- (.Location (Math|Transform|BreakTransform (LocalVariables|GetTargetPosition))) (LocalVariables|GetCurrentLocation)) (LocalVariables|GetScaleFactor))) (.rotation (LocalVariables|GetTargetPosition)) (.scale (LocalVariables|GetTargetPosition))) (.interpolatedlocation Leg) (.offset Leg) (.progress Leg) (.previousprogress Leg) (.placementoffset Leg) StepLength) true))))

(fn AdjustStepDirection
  (params (leg :type S%20Calculated%20Leg%20Info%20Structure) (BoneName :type Name))
  (bind (_lockedworldtransform _targetworldtransform _interpolatedlocation _offset _progress _previousprogress _placementoffset _steplength) (Utilities|Struct|BreakS_CalculatedLegInfo leg))
  (bind (_location _rotation _scale) (Math|Transform|BreakTransform _targetworldtransform))
  (LocalVariables|SetStartLocation (.location (Helpers|ToWorld (.Value (Utilities|Map|Find (Variables|Private/Global|GetActorLegInitialLocalTransform) BoneName)))))
  (LocalVariables|SetTargetLocation (.Location (Math|Transform|BreakTransform (.TargetWorldTransform (Utilities|Struct|BreakS_CalculatedLegInfo leg)))))
  (LocalVariables|SetTargetLength (Math|Vector|VectorLength (- (LocalVariables|GetTargetLocation) (LocalVariables|GetStartLocation))))
  (LocalVariables|SetRemapedTargetLocation (+ (LocalVariables|GetStartLocation) (* (Math|Vector|Normalize (Variables|Private/Global|GetVelocity)) (LocalVariables|GetTargetLength))))
  (CallFunction|PrintTextLog (Utilities|Array|MakeArray (Utilities|String|ToString(Float) (CallFunction|GetAngleBetween (- (LocalVariables|GetTargetLocation) (LocalVariables|GetStartLocation)) (Variables|Private/Global|GetVelocity))) "angle") "ang diff" 2.0 "(R=0.000000,G=0.855387,B=1.000000,A=1.000000)")
  (if (< (CallFunction|GetAngleBetween (- (LocalVariables|GetTargetLocation) (LocalVariables|GetStartLocation)) (Variables|Private/Global|GetVelocity)) 1e+01)
    (return leg false)
    (else
      (Utilities|FlowControl|Sequence
        (:then_0
          (if (> (CallFunction|GetAngleBetween (- (LocalVariables|GetTargetLocation) (LocalVariables|GetStartLocation)) (Variables|Private/Global|GetVelocity)) 4e+01)
            _))
        (:then_1
          (return (Utilities|Struct|MakeS_CalculatedLegInfo _lockedworldtransform (Math|Transform|MakeTransform (Math|Vector|Lerp(Vector) (LocalVariables|GetTargetLocation) (LocalVariables|GetRemapedTargetLocation) 0.5) _rotation _scale) _interpolatedlocation _offset _progress _previousprogress _placementoffset _steplength) true))))))

(fn InterpolateLegTarget
  (params (Leg :type S%20Calculated%20Leg%20Info%20Structure) (BoneName :type Name))
  (bind (_updatedleg _isupdated) (Calculation/Leg|RemapStepLength Leg (Variables|Private/Step|GetStepLength)))
  (bind (_updatedleg_2 _ischanged) (Calculation/Leg|AdjustStepDirection _updatedleg BoneName))
  (LocalVariables|SetTarget (.TargetWorldTransform (Utilities|Struct|BreakS_CalculatedLegInfo _updatedleg_2)))
  (Utilities|FlowControl|Sequence
    (:then_0
      (if (or _ischanged _isupdated)
        (bind _outtransform (Helpers|TraceatLocation (LocalVariables|GetTarget)))
        (LocalVariables|SetTarget _outtransform)))
    (:then_1
      (return (.LockedWorldTransform (Utilities|Struct|BreakS_CalculatedLegInfo _updatedleg_2)) (LocalVariables|GetTarget) (.StepLength (Utilities|Struct|BreakS_CalculatedLegInfo _updatedleg_2))))))