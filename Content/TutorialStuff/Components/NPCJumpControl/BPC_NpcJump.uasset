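; NPC jump component that launches its owning Character toward a given destination.
; JumpTo computes a ballistic launch velocity over JumpDuration with approximate gravity, taking target height from a WorldStatic sphere trace or the destination.
; A self-calling delayed event then re-launches horizontally while falling to converge within 70% of that duration, preserving vertical velocity.
; Horizontal movement stops once the character reaches the destination in 2D.
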(event Custom|TrackJumpPositionTick
  (bind _owningcharacter (Variables|Default|GetOwningCharacter))
  (bind _destination (Variables|Default|GetDestination))
  (bind _returnvalue (Transformation|GetActorLocation _owningcharacter))
  ;[0.15 0.15 0.15 0.5] Wait as first tick because we won't be jumping right away.
  (Utilities|FlowControl|Delay (Variables|Default|GetJumpTickDuration))
  (Variables|Default|SetJumpTimeLeft (- (Variables|Default|GetJumpTimeLeft) (Variables|Default|GetJumpTickDuration)))
  (if (and (AI|Components|NavMovement|IsFalling (Variables|/Script/Engine.Character|GetCharacterMovement (Variables|Default|GetOwningCharacter))) (> (Variables|Default|GetJumpTimeLeft) 0.0001))
    (if (> (Math|Vector|Distance2D(Vector) _destination _returnvalue) 1.0)
      (Character|LaunchCharacter (Variables|Default|GetOwningCharacter) (Math|Vector|MakeVector (.X (Math|Vector|BreakVector (/ (/ (- _destination _returnvalue) (/ (Variables|Default|GetJumpTimeLeft) (Variables|Default|GetJumpTickDuration))) (Variables|Default|GetJumpTickDuration)))) (.Y (Math|Vector|BreakVector (/ (/ (- _destination _returnvalue) (/ (Variables|Default|GetJumpTimeLeft) (Variables|Default|GetJumpTickDuration))) (Variables|Default|GetJumpTickDuration)))) 0.0) true false)
      (CallFunction|TrackJumpPositionTick)
      (else
        ;[0.15 0.15 0.15 0.5] Stop horizontal movement
        (Character|LaunchCharacter (Variables|Default|GetOwningCharacter) "0, 0, 0" true false)))))

(event EventBeginPlay
  (bind _ascharacter (Utilities|Casting|CastToCharacter (Components|GetOwner)))
  (Variables|Default|SetOwningCharacter _ascharacter))

(event EventTick
  (params (DeltaSeconds :type Float%20%28single-precision%29)))

(fn Jumpto
  (params (DestinationJump :type Vector))
  (if (Character|CanJump (Variables|Default|GetOwningCharacter))
    (Variables|Default|SetDestination DestinationJump)
    (bind _velocity (Private|GetJumpInitialVelocity))
    (Character|LaunchCharacter (Variables|Default|GetOwningCharacter) _velocity true true)
    (Variables|Default|SetJumpTimeLeft (* (Variables|Default|GetJumpDuration) 0.7))
    (CallFunction|TrackJumpPositionTick)
    (return true)
    (else
      (return false))))

(fn GetJumpInitialVelocity
  (bind _owningcharacter (Variables|Default|GetOwningCharacter))
  (bind _charactermovement (Variables|/Script/Engine.Character|GetCharacterMovement _owningcharacter))
  (bind _returnvalue (Class|CharacterMovementComponent|GetMaxJumpHeight _charactermovement))
  (bind _returnvalue_2 (* _returnvalue 2.0))
  (LocalVariables|SetStartLocation (Transformation|GetActorLocation (Variables|Default|GetOwningCharacter)))
  (LocalVariables|SetLocationDelta (- (Variables|Default|GetDestination) (LocalVariables|GetStartLocation)))
  (Utilities|FlowControl|Sequence
    (:then_0
      (bind (_outhit _returnvalue_3) (Collision|SphereTraceForObjects (+ (LocalVariables|GetStartLocation) (Math|Vector|MakeVector 0.0 0.0 _returnvalue_2)) (- (LocalVariables|GetStartLocation) (Math|Vector|MakeVector 0.0 0.0 _returnvalue_2)) (Math|Vector|VectorLength (LocalVariables|GetLocationDelta)) (Utilities|Array|MakeArray "ObjectTypeQuery1") false 0 "None"))
      (if _returnvalue_3
        (LocalVariables|SetTargetZ (.Z (Math|Vector|BreakVector (.Location (Collision|BreakHitResult _outhit)))))
        (else
          (LocalVariables|SetTargetZ (.z (Variables|Default|GetDestination))))))
    (:then_1
      (return false (/ (Math|Vector|MakeVector (.X (Math|Vector|BreakVector (LocalVariables|GetLocationDelta))) (.Y (Math|Vector|BreakVector (LocalVariables|GetLocationDelta))) (- (LocalVariables|GetTargetZ) (+ (.z (LocalVariables|GetStartLocation)) (* (Math|Float|Square (Variables|Default|GetJumpDuration)) -0.5 1e+03)))) (Variables|Default|GetJumpDuration))))))