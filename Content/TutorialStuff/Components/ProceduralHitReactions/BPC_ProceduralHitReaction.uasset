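; Actor component that gives its owner procedural hit reactions through partial physics simulation on the skeletal mesh.
; ReactToDamage picks the allowed bone nearest the damage location, then simulates it and any forced bones with a damage-scaled impulse away from the hit.
; A self-calling delayed event steps physics blend weight down.
; A retriggerable timer restores query-only, non-simulated state after the reaction, unless the owner is dead.
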(event Custom|ProcessDamageTimer
  (bind _returnvalue (Components|GetOwner))
  (Variables|Default|SetIsBeingDamaged true)
  (Utilities|FlowControl|RetriggerableDelay (Variables|Default|GetReactionDuration))
  (bind _isdead (Class|PBIDamageable|GetIsDead(Message) _returnvalue))
  (if (not _isdead)
    (bind _skeletalmeshcomponent (Class|BPIwithSkeletalMeshComponent|GetSkeletalMeshComponent(Message) _returnvalue))
    (Utilities|IsValid _skeletalmeshcomponent
      (:Is%20Valid
        (Collision|SetCollisionEnabled _skeletalmeshcomponent "QueryOnly")
        (Class|SkeletalMeshComponent|SetAllBodiesSimulatePhysics _skeletalmeshcomponent false)
        (Class|SkeletalMeshComponent|SetAllBodiesPhysicsBlendWeight _skeletalmeshcomponent 0.0 false)
        (Variables|Default|SetIsBeingDamaged false)))))

(event Custom|ProcessBoneBlend
  (params (Mesh :type Skeletal%20Mesh%20Component%20Object%20Reference) (BlendDecrement :type Float%20%28double-precision%29) (CurrentBlend :type Float%20%28double-precision%29) (ShouldContinue :type Boolean))
  (if ShouldContinue
    (bind (_updatedincrement _updatedvalue _shouldcontinue) (CallFunction|EvalBoneBlend Mesh BlendDecrement CurrentBlend))
    (Utilities|FlowControl|RetriggerableDelay (Variables|Default|GetInterpTime))
    (CallFunction|ProcessBoneBlend Mesh _updatedincrement _updatedvalue _shouldcontinue)))

(event EventBeginPlay)

(event EventTick
  (params (DeltaSeconds :type Float%20%28single-precision%29)))

(fn ReacttoDamage
  (params (Damage :type S%20Damage%20Info%20Structure))
  (Utilities|FlowControl|Sequence
    (:then_0
      (bind _skeletalmeshcomponent (Class|BPIwithSkeletalMeshComponent|GetSkeletalMeshComponent(Message) (Components|GetOwner)))
      (bind _output_get (LocalVariables|SetMesh _skeletalmeshcomponent))
      (Utilities|IsValid _output_get
        (:Is%20Not%20Valid
          (return))))
    (:then_1
      (LocalVariables|SetImpule (* (Math|Vector|Normalize (- (Transformation|GetActorLocation (Components|GetOwner)) (.damagelocation Damage))) (.damageamount Damage) 10)))
    (:then_2
      (bind (_bone_name _isfound) (CallFunction|GetHitBone Damage (LocalVariables|GetMesh)))
      (if _isfound
        (CallFunction|BoneReactDamage (LocalVariables|GetMesh) _bone_name (LocalVariables|GetImpule))))
    (:then_3
      (for _array_element (Variables|Default|GetForcedBones)
        (CallFunction|BoneReactDamage (LocalVariables|GetMesh) _array_element (LocalVariables|GetImpule))))))

(fn GetHitBone
  (params (Damage :type S%20Damage%20Info%20Structure) (Mesh :type Skeletal%20Mesh%20Component%20Object%20Reference))
  (for _array_element (Variables|Default|GetAllowedBones)
    (if (or (< (Math|Vector|VectorLength (- (.damagelocation Damage) (Transformation|GetSocketLocation Mesh _array_element))) (LocalVariables|GetBestDistance)) (< (LocalVariables|GetBestDistance) 0.0))
      (LocalVariables|SetBestDistance (Math|Vector|VectorLength (- (.damagelocation Damage) (Transformation|GetSocketLocation Mesh _array_element))))
      (LocalVariables|SetBestBoneName _array_element)
      (LocalVariables|SetIsSelected true)))
  (return (LocalVariables|GetBestBoneName) (LocalVariables|GetIsSelected)))

(fn BoneReactDamage
  (params (Mesh :type Skeletal%20Mesh%20Component%20Object%20Reference) (InBoneName :type Name%20%28by%20ref%29) (Impulse :type Vector))
  (Collision|SetCollisionEnabled Mesh "QueryAndPhysics")
  (Class|SkeletalMeshComponent|SetAllBodiesBelowSimulatePhysics Mesh InBoneName true true)
  (Physics|AddImpulse Mesh Impulse InBoneName true)
  (Class|SkeletalMeshComponent|SetAllBodiesBelowPhysicsBlendWeight Mesh InBoneName (Variables|Default|GetMaxBlend) false true)
  (CallFunction|ProcessDamageTimer)
  (CallFunction|ProcessBoneBlend Mesh (* (/ (Variables|Default|GetMaxBlend) (- (Variables|Default|GetReactionDuration) 0.1)) (Variables|Default|GetInterpTime)) (Variables|Default|GetMaxBlend) true))

(fn EvalBoneBlend
  (params (Mesh :type Skeletal%20Mesh%20Component%20Object%20Reference) (Decrement :type Float%20%28double-precision%29) (CurrentValue :type Float%20%28double-precision%29))
  (if (Variables|Default|GetIsBeingDamaged)
    (Utilities|IsValid Mesh
      (:Is%20Valid
        (bind _isdead (Class|PBIDamageable|GetIsDead(Message) (Components|GetOwner)))
        (if _isdead
          _
          (else
            (bind _output_get (LocalVariables|SetBlendValue (- CurrentValue Decrement)))
            (Class|SkeletalMeshComponent|SetAllBodiesPhysicsBlendWeight Mesh _output_get false)
            (if (<= (LocalVariables|GetBlendValue) 0.0)
              (return 0.0 0.0 false)
              (else
                (return Decrement (LocalVariables|GetBlendValue) true))))))
      (:Is%20Not%20Valid
        _)))
  (return 0.0 0.0 false))