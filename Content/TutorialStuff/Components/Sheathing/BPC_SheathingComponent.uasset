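; Character component that draws and sheathes weapons between sheath and arm child-actor slots.
; Requests check slot occupancy and whether a change is allowed, then play the weapon's montage, or swap instantly without one.
; A Weapon Change notify moves the actor class between slots, applies weapon info to the character and releases the change lock, so a following change can interrupt the montage.
; Completion or interruption broadcasts the result.
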(event Custom|PlayDrawAnimation
  (params (WeaponInfo :type S%20Armed%20Weapon%20Info%20Structure) (ArmSlot :type Child%20Actor%20Component%20Object%20Reference) (SheathSlot :type Child%20Actor%20Component%20Object%20Reference))
  (bind _unsheatheanimation (Utilities|Struct|BreakS_ArmedWeaponInfo WeaponInfo))
  (Utilities|IsValid _unsheatheanimation
    (:Is%20Valid
      (Utilities|IsValid (Variables|Default|GetOwnerCharacter)
        (:Is%20Valid
          (bind _notifyname (Animation|Montage|PlayMontage (Variables|/Script/Engine.Character|GetMesh (Variables|Default|GetOwnerCharacter)) _unsheatheanimation)
            (:then
              (Variables|Default|SetIsPlayingSheathingMontage true)
              (Private|StartWeaponChange))
            (:OnCompleted
              (Variables|Default|SetIsPlayingSheathingMontage false)
              (Private|FinishWeaponChange)
              (Default|CallOnWeaponChangeDone true))
            (:OnInterrupted
              (Private|InterruptWeaponChange SheathSlot ArmSlot))
            (:OnNotifyBegin
              (switch name _notifyname
                (:WeaponChange
                  (Private|DrawWeaponPrivate WeaponInfo ArmSlot SheathSlot))))))))
    (:Is%20Not%20Valid
      ;[0.15 0.15 0.15 0.5] If no amination, just place it in the hand
      (bind _issuccess (Private|DrawWeaponPrivate WeaponInfo ArmSlot SheathSlot))
      (Default|CallOnWeaponChangeDone _issuccess))))

(event Custom|PlaySheatheAnimation
  (params (Weapon%20Info :type S%20Armed%20Weapon%20Info%20Structure) (ArmSlot :type Child%20Actor%20Component%20Object%20Reference) (SheatheSlot :type Child%20Actor%20Component%20Object%20Reference))
  (bind _sheatheanimation (Utilities|Struct|BreakS_ArmedWeaponInfo Weapon%20Info))
  (Utilities|IsValid _sheatheanimation
    (:Is%20Valid
      (Utilities|IsValid (Variables|Default|GetOwnerCharacter)
        (:Is%20Valid
          (bind _notifyname (Animation|Montage|PlayMontage (Variables|/Script/Engine.Character|GetMesh (Variables|Default|GetOwnerCharacter)) _sheatheanimation)
            (:then
              (Variables|Default|SetIsPlayingSheathingMontage true)
              (Private|StartWeaponChange))
            (:OnCompleted
              (Variables|Default|SetIsPlayingSheathingMontage false)
              (Private|FinishWeaponChange)
              (Default|CallOnWeaponChangeDone true))
            (:OnInterrupted
              (Private|InterruptWeaponChange ArmSlot SheatheSlot))
            (:OnNotifyBegin
              (switch name _notifyname
                (:WeaponChange
                  (Private|SheafeWeaponPrivate ArmSlot SheatheSlot))))))))
    (:Is%20Not%20Valid
      ;[0.15 0.15 0.15 0.5] If no amination, just place it in the sheathe
      (bind _issuccess (Private|SheafeWeaponPrivate ArmSlot SheatheSlot))
      (Default|CallOnWeaponChangeDone _issuccess))))

(event EventBeginPlay
  (bind _ascharacter (Utilities|Casting|CastToCharacter (Components|GetOwner)))
  (Variables|Default|SetOwnerCharacter _ascharacter))

(event EventTick
  (params (DeltaSeconds :type Float%20%28single-precision%29)))

(fn DrawWeapon
  (params (WeaponToDraw :type S%20Armed%20Weapon%20Info%20Structure) (ArmSlot :type Child%20Actor%20Component%20Object%20Reference) (SheathSlot :type Child%20Actor%20Component%20Object%20Reference))
  (Utilities|FlowControl|Sequence
    (:then_0
      (bind _canchange (CallFunction|CheckCanChangeWeapon))
      (if (not _canchange)
        (return false)))
    (:then_1
      ;[0.15 0.15 0.15 0.5] Can't change if slot is taken
      (Utilities|IsValid ArmSlot
        (:Is%20Valid
          (Utilities|IsValid (Variables|/Script/Engine.ChildActorComponent|GetChildActor ArmSlot)
            (:Is%20Valid
              (return false))))
        (:Is%20Not%20Valid
          (return false))))
    (:then_2
      (Utilities|IsValid SheathSlot
        (:Is%20Valid
          (if (Utilities|DoesObjectImplementInterface (Variables|/Script/Engine.ChildActorComponent|GetChildActor SheathSlot) "/Game/TutorialStuff/Items/BaseWeapon/BPI_Weapon.BPI_Weapon_C")
            (CallFunction|PlayDrawAnimation WeaponToDraw ArmSlot SheathSlot)
            (return true)
            (else
              (return false))))
        (:Is%20Not%20Valid
          (return false))))))

(fn SheatheWeapon
  (params (Weapon%20Info :type S%20Armed%20Weapon%20Info%20Structure) (SheathSlot :type Child%20Actor%20Component%20Object%20Reference) (ArmSlot :type Child%20Actor%20Component%20Object%20Reference) (IsForced :type Boolean))
  (Utilities|FlowControl|Sequence
    (:then_0
      (bind _canchange (CallFunction|CheckCanChangeWeapon))
      (if (not _canchange)
        (return false)))
    (:then_1
      (Utilities|IsValid SheathSlot
        (:Is%20Valid
          (Utilities|IsValid (Variables|/Script/Engine.ChildActorComponent|GetChildActor SheathSlot)
            (:Is%20Valid
              (return false))))))
    (:then_2
      ;[0.15 0.15 0.15 0.5] TODO
      (if IsForced
        (return false)))
    (:then_3
      (Utilities|IsValid ArmSlot
        (:Is%20Valid
          (if (Utilities|DoesObjectImplementInterface (Variables|/Script/Engine.ChildActorComponent|GetChildActor ArmSlot) "/Game/TutorialStuff/Items/BaseWeapon/BPI_Weapon.BPI_Weapon_C")
            (CallFunction|PlaySheatheAnimation Weapon%20Info ArmSlot SheathSlot)
            (return true)
            (else
              (return false))))
        (:Is%20Not%20Valid
          (return false))))))

(fn CheckCanChangeWeapon
  (bind _ownercharacter (Variables|Default|GetOwnerCharacter))
  (if (Variables|Default|GetIsChangingWeapon)
    (return false)
    (else
      ;[0.15 0.15 0.15 0.5] Force allow if plaing montage, because previous check has passed, and we considering consequent sheafing to be the same action. but montage may prevent playing it, we allow to interrupt in between
      (if (Variables|Default|GetIsPlayingSheathingMontage)
        (return true)
        (else
          (Utilities|IsValid _ownercharacter
            (:Is%20Valid
              (bind _canchangeweapon (Class|BPIArmed|CheckCanChangeWeapon(Message) _ownercharacter))
              (return _canchangeweapon))))))))

(fn DrawWeaponPrivate
  (params (WeaponToDraw :type S%20Armed%20Weapon%20Info%20Structure) (ArmSlot :type Child%20Actor%20Component%20Object%20Reference) (SheathSlot :type Child%20Actor%20Component%20Object%20Reference))
  (bind _childactor (Variables|/Script/Engine.ChildActorComponent|GetChildActor SheathSlot))
  (Utilities|FlowControl|Sequence
    (:then_0
      ;[0.15 0.15 0.15 0.5] Can't change if slot is taken
      (Utilities|IsValid ArmSlot
        (:Is%20Valid
          (Utilities|IsValid (Variables|/Script/Engine.ChildActorComponent|GetChildActor ArmSlot)
            (:Is%20Valid
              _)))
        (:Is%20Not%20Valid
          _))
      (Private|InterruptWeaponChange :!label _label)
      (return false))
    (:then_1
      (Utilities|IsValid SheathSlot
        (:Is%20Valid
          (Utilities|IsValid _childactor
            (:Is%20Valid
              (LocalVariables|SetWeaponClass (Utilities|GetClass _childactor)))
            (:Is%20Not%20Valid
              (goto _label))))
        (:Is%20Not%20Valid
          (goto _label))))
    (:then_2
      (Utilities|IsValid ArmSlot
        (:Is%20Not%20Valid
          (goto _label))))
    (:then_3
      (ChildActorComponent|SetChildActorClass SheathSlot 0)
      (ChildActorComponent|SetChildActorClass ArmSlot (LocalVariables|GetWeaponClass))
      (bind _output_get (LocalVariables|SetWeaponActor (Variables|/Script/Engine.ChildActorComponent|GetChildActor ArmSlot)))
      (Actor|SetOwner _output_get (Variables|Default|GetOwnerCharacter)))
    (:then_4
      (Class|BPIArmed|ApplyWeapon(Message) (Variables|Default|GetOwnerCharacter) WeaponToDraw (LocalVariables|GetWeaponActor))
      (Private|FinishWeaponChange)
      (Default|CallOnWeaponDrawn)
      (return true))))

(fn SheafeWeaponPrivate
  (params (ArmSlot :type Child%20Actor%20Component%20Object%20Reference) (SheathSlot :type Child%20Actor%20Component%20Object%20Reference))
  (bind _childactor (Variables|/Script/Engine.ChildActorComponent|GetChildActor ArmSlot))
  (Utilities|FlowControl|Sequence
    (:then_0
      ;[0.15 0.15 0.15 0.5] Can't change if slot is taken
      (Utilities|IsValid SheathSlot
        (:Is%20Valid
          (Utilities|IsValid (Variables|/Script/Engine.ChildActorComponent|GetChildActor SheathSlot)
            (:Is%20Valid
              _)))
        (:Is%20Not%20Valid
          _))
      (Private|InterruptWeaponChange :!label _label)
      (return false))
    (:then_1
      (Utilities|IsValid ArmSlot
        (:Is%20Valid
          (Utilities|IsValid _childactor
            (:Is%20Valid
              (LocalVariables|SetWeaponClass (Utilities|GetClass _childactor)))
            (:Is%20Not%20Valid
              (goto _label))))
        (:Is%20Not%20Valid
          (goto _label))))
    (:then_2
      (Utilities|IsValid ArmSlot
        (:Is%20Not%20Valid
          (goto _label))))
    (:then_3
      (ChildActorComponent|SetChildActorClass ArmSlot 0)
      (ChildActorComponent|SetChildActorClass SheathSlot (LocalVariables|GetWeaponClass)))
    (:then_4
      (Class|BPIArmed|ApplyWeapon(Message) (Variables|Default|GetOwnerCharacter) (Utilities|Struct|MakeS_ArmedWeaponInfo (LocalVariables|GetEmptyArray) 0 0 0.0))
      (Private|FinishWeaponChange)
      (Default|CallOnWeaponSheathed)
      (return true))))

(fn StartWeaponChange
  (Variables|Default|SetIsChangingWeapon true))

(fn FinishWeaponChange
  (Variables|Default|SetIsChangingWeapon false))

(fn InterruptWeaponChange
  (params (EmptySlot :type Child%20Actor%20Component%20Object%20Reference) (PopulatedSlot :type Child%20Actor%20Component%20Object%20Reference))
  (Utilities|FlowControl|Sequence
    (:then_0
      (Variables|Default|SetIsPlayingSheathingMontage false))
    (:then_1
      (Utilities|IsValid EmptySlot
        (:Is%20Valid
          (Utilities|IsValid (Variables|/Script/Engine.ChildActorComponent|GetChildActor EmptySlot)
            (:Is%20Not%20Valid
              (Utilities|IsValid PopulatedSlot
                (:Is%20Valid
                  (Utilities|IsValid (Variables|/Script/Engine.ChildActorComponent|GetChildActor PopulatedSlot)
                    (:Is%20Valid
                      (LocalVariables|SetIsSuccessful true))))))))))
    (:then_2
      (Private|FinishWeaponChange))
    (:then_3
      (Default|CallOnWeaponChangeDone (LocalVariables|GetIsSuccessful)))))