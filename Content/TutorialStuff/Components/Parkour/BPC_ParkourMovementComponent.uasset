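; Parkour actor component that lets its owning character climb, mantle or vault over obstacles ahead.
; Parkour() tries climb, mantle, then vault, using sphere and line traces to find ledges, landings and clearance, producing named warp points.
; A successful move disables collision, switches to Flying, feeds Motion Warping targets and plays the montage, then restores collision and Walking when it ends.
; Owner components come through interface messages, and dispatchers signal parkour start and end.
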(event Custom|EndVault
  ;[0.15 0.15 0.15 0.5] End Animation
  (Variables|Default|SetIsVaulting false)
  (Collision|SetActorEnableCollision (Variables|Default|GetOwner) true)
  (bind _charactermovementcomponent (PrivateGetters|GetCharacterMovementComponent))
  (Pawn|Components|CharacterMovement|SetMovementMode _charactermovementcomponent "MOVE_Walking" 0)
  (Default|CallOnParkourEnd))

(event Custom|Start%20Parkour%20Vault
  (params (WarpPoints :type Array%20of%20PMC%20Warp%20Point%20Structures) (Montage :type Anim%20Montage%20Object%20Reference))
  ;[0.15 0.15 0.15 0.5] Full parkour cycle
  (Utilities|FlowControl|Sequence
    (:then_0
      (PrivateParkour|StartParkour))
    (:then_1
      (PrivateParkour|SetVaultMotionWarp WarpPoints))
    (:then_2
      (bind _mesh (PrivateGetters|GetCharacterSkeletalMeshComponent))
      (Animation|Montage|PlayMontage _mesh Montage
        (:OnCompleted
          _)
        (:OnInterrupted
          _))
      (CallFunction|EndVault))
    (:then_3
      (Variables|Default|SetIsVaulting true))))

(event EventBeginPlay
  (Variables|Default|SetOwner (Components|GetOwner)))

(event EventTick
  (params (DeltaSeconds :type Float%20%28single-precision%29)))

(fn GetCharacterMovementComponent
  (bind _movementcomponent (Class|BPIMovableCharacter|GetCharacterMovementComponent(Message) (Variables|Default|GetOwner)))
  (return _movementcomponent))

(fn GetCharacterSkeletalMeshComponent
  (bind _skeletalmeshcomponent (Class|BPIwithSkeletalMeshComponent|GetSkeletalMeshComponent(Message) (Variables|Default|GetOwner)))
  (return _skeletalmeshcomponent))

(fn GetMotionWarpingComponent
  (bind _motionwarping (Class|BPIwithMotionWarpingComponent|GetWarpingComponent(Message) (Variables|Default|GetOwner)))
  (return _motionwarping))

(fn GetOwnerActor
  (return (Components|GetOwner)))

(fn GetCanVault
  (if (Variables|Default|GetIsVaulting)
    (return false)
    (else
      (bind _charactermovementcomponent (PrivateGetters|GetCharacterMovementComponent))
      (Utilities|IsValid _charactermovementcomponent
        (:Is%20Valid
          (if (AI|Components|NavMovement|IsFalling _charactermovementcomponent)
            (return false)
            (else
              (return true))))
        (:Is%20Not%20Valid
          (return false))))))

(fn GetCanClimb
  (bind _owner (Variables|Default|GetOwner))
  (bind _returnvalue (Transformation|GetActorLocation _owner))
  (if (Variables|Default|GetIsVaulting)
    (return false)
    (elif (< (Math|Vector|VectorLength (Transformation|GetVelocity (Variables|Default|GetOwner))) 1.2e+03)
      ;[0.15 0.15 0.15 0.5] Check if there is an obsticale on top. Required because extends over the head
      (bind _returnvalue_2 (Collision|MultiSphereTraceByChannel _returnvalue (+ _returnvalue "0.000000,0.000000,230.000000") 1e+01 "TraceTypeQuery1" false 0 "None"))
      (return (not _returnvalue_2))
      (else
        (return false)))))

(fn GetVaultOverPosition
  (Utilities|IsValid (Variables|Default|GetOwner)
    (:Is%20Valid
      (Utilities|FlowControl|Sequence
        (:then_0
          (LocalVariables|SetActorForwardVector (Transformation|GetActorForwardVector (Variables|Default|GetOwner))))
        (:then_1
          (LocalVariables|SetActorLocation (Transformation|GetActorLocation (Variables|Default|GetOwner))))
        (:then_2
          ;[1 1 1] Seatching For an obsticle to vault over
          (bind _index (Utilities|FlowControl|ForLoopwithBreak 0 1 :!label _label)
            (:LoopBody
              (bind (_outhit _returnvalue) (Collision|SphereTraceByChannel (+ (LocalVariables|GetActorLocation) (Math|Vector|MakeVector 0.0 0.0 (* _index 30))) (+ (+ (LocalVariables|GetActorLocation) (Math|Vector|MakeVector 0.0 0.0 (* _index 30))) (* (LocalVariables|GetActorForwardVector) 2.5e+02)) 5.0 "TraceTypeQuery1" false 0 "None" true "(R=1.000000,G=0.680251,B=0.000000,A=1.000000)" "(R=0.000000,G=0.971714,B=1.000000,A=1.000000)"))
              (if _returnvalue
                (Utilities|FlowControl|Sequence
                  (:then_0
                    (goto _label Break))
                  (:then_1
                    ;[1 1 1] Getting vault points
                    (bind _index_2 (Utilities|FlowControl|ForLoopwithBreak 0 5 :!label _label_2)
                      (:LoopBody
                        (bind (_outhit_2 _returnvalue_2) (Collision|SphereTraceByChannel (+ (* (* _index_2 50) (LocalVariables|GetActorForwardVector)) (+ (.ImpactPoint (Collision|BreakHitResult _outhit)) "0.000000,0.000000,60.000000")) (- (+ (* (* _index_2 50) (LocalVariables|GetActorForwardVector)) (+ (.ImpactPoint (Collision|BreakHitResult _outhit)) "0.000000,0.000000,60.000000")) "0.000000,0.000000,100.000000") 1e+01 "TraceTypeQuery1" false 0 "None" true "(R=0.125059,G=0.000000,B=1.000000,A=1.000000)" "(R=1.000000,G=0.856791,B=0.000000,A=1.000000)"))
                        (if _returnvalue_2
                          (Utilities|FlowControl|Sequence
                            (:then_0
                              (if (== _index_2 0)
                                (LocalVariables|SetVaultStartPosition (.ImpactPoint (Collision|BreakHitResult _outhit_2)))))
                            (:then_1
                              (LocalVariables|SetVaultJumpOffPosition (.ImpactPoint (Collision|BreakHitResult _outhit_2)))))
                          (else
                            (Utilities|FlowControl|Sequence
                              (:then_0
                                ;[1 1 1] can land??
                                (bind (_outhit_3 _returnvalue_3) (Collision|LineTraceByChannel (+ (.TraceStart (Collision|BreakHitResult _outhit_2)) (* (LocalVariables|GetActorForwardVector) 8e+01)) (- (+ (.TraceStart (Collision|BreakHitResult _outhit_2)) (* (LocalVariables|GetActorForwardVector) 8e+01)) "0.000000,0.000000,200.000000") "TraceTypeQuery1" false 0 "None"))
                                (if _returnvalue_3
                                  (if (< (Math|Vector|VectorLength (- (LocalVariables|GetVaultStartPosition) (.Location (Collision|BreakHitResult _outhit_3)))) 3e+02)
                                    (LocalVariables|SetVaultLandPosition (+ (.Location (Collision|BreakHitResult _outhit_3)) (* (LocalVariables|GetActorForwardVector) 1.5e+02)))
                                    (else
                                      (LocalVariables|SetVaultLandPosition "0, 0, 0")))
                                  ;[1 1 1] can jump through?
                                  (bind _index_3 (Utilities|FlowControl|ForLoopwithBreak 1 3)
                                    (:LoopBody
                                      (bind _returnvalue_4 (Collision|SphereTraceByChannel (Math|Vector|MakeVector (.x (+ (LocalVariables|GetVaultStartPosition) (Math|Vector|MakeVector 0.0 0.0 (+ (* _index_3 35) 15.0)))) (.y (+ (LocalVariables|GetVaultStartPosition) (Math|Vector|MakeVector 0.0 0.0 (+ (* _index_3 35) 15.0)))) (.z (+ (LocalVariables|GetVaultStartPosition) (Math|Vector|MakeVector 0.0 0.0 (+ (* _index_3 35) 15.0))))) (Math|Vector|MakeVector (.x (LocalVariables|GetVaultLandPosition)) (.y (LocalVariables|GetVaultLandPosition)) (.z (+ (LocalVariables|GetVaultStartPosition) (Math|Vector|MakeVector 0.0 0.0 (+ (* _index_3 35) 15.0))))) 32.0 "TraceTypeQuery1" false 0 "None" true "(R=1.000000,G=0.680251,B=0.000000,A=1.000000)" "(R=0.000000,G=0.971714,B=1.000000,A=1.000000)"))
                                      (if _returnvalue_4
                                        (return false 0)))
                                    (:Completed
                                      (return true (Utilities|Array|MakeArray (Utilities|Struct|MakePMC_WarpPoint "VaultStart" (LocalVariables|GetVaultStartPosition) "0.000000,0.000000,0.000000") (Utilities|Struct|MakePMC_WarpPoint "VaultJumpOff" (LocalVariables|GetVaultJumpOffPosition) "0.000000,0.000000,0.000000") (Utilities|Struct|MakePMC_WarpPoint "VaultLand" (LocalVariables|GetVaultLandPosition) "0.000000,0.000000,0.000000")))))))
                              (:then_1
                                (goto _label_2 Break)))))))))))
            (:Completed
              (return false 0))))))
    (:Is%20Not%20Valid
      (return false 0))))

(fn GetMantlePosition
  (Utilities|IsValid (Variables|Default|GetOwner)
    (:Is%20Valid
      (Utilities|FlowControl|Sequence
        (:then_0
          (LocalVariables|SetActorForwardVector (Transformation|GetActorForwardVector (Variables|Default|GetOwner))))
        (:then_1
          (LocalVariables|SetActorLocation (Transformation|GetActorLocation (Variables|Default|GetOwner))))
        (:then_2
          ;[1 1 1] Seatching For an obsticle to vault over
          (bind _index (Utilities|FlowControl|ForLoopwithBreak 0 2 :!label _label)
            (:LoopBody
              (bind (_outhit _returnvalue) (Collision|SphereTraceByChannel (+ (LocalVariables|GetActorLocation) (Math|Vector|MakeVector 0.0 0.0 (* _index 30))) (+ (+ (LocalVariables|GetActorLocation) (Math|Vector|MakeVector 0.0 0.0 (* _index 30))) (* (LocalVariables|GetActorForwardVector) 6e+01)) 5.0 "TraceTypeQuery1" false 0 "None" true "(R=1.000000,G=0.680251,B=0.000000,A=1.000000)" "(R=0.000000,G=0.971714,B=1.000000,A=1.000000)"))
              (if _returnvalue
                (Utilities|FlowControl|Sequence
                  (:then_0
                    (goto _label Break))
                  (:then_1
                    ;[1 1 1] Getting vault start
                    (LocalVariables|SetMantleStartAngle (Math|Rotator|MakeRotfromX (* (.ImpactNormal (Collision|BreakHitResult _outhit)) -1.0)))
                    (bind (_outhit_2 _returnvalue_2) (Collision|SphereTraceByChannel (+ (.ImpactPoint (Collision|BreakHitResult _outhit)) "0.000000,0.000000,20.000000") (- (+ (.ImpactPoint (Collision|BreakHitResult _outhit)) "0.000000,0.000000,20.000000") "0.000000,0.000000,100.000000") 1e+01 "TraceTypeQuery1" false 0 "None" true "(R=0.125059,G=0.000000,B=1.000000,A=1.000000)" "(R=1.000000,G=0.856791,B=0.000000,A=1.000000)"))
                    (if _returnvalue_2
                      (LocalVariables|SetMantleStartPosition (- (.ImpactPoint (Collision|BreakHitResult _outhit_2)) (* (LocalVariables|GetActorForwardVector) 40)))
                      ;[0.15 0.15 0.15 0.5] get vault end
                      (bind _index_2 (Utilities|FlowControl|ForLoopwithBreak 1 3 :!label _label_2)
                        (:LoopBody
                          (bind (_outhit_3 _returnvalue_3) (Collision|LineTraceByChannel (+ (.TraceStart (Collision|BreakHitResult _outhit_2)) (* (* _index_2 25) (LocalVariables|GetActorForwardVector))) (- (+ (.TraceStart (Collision|BreakHitResult _outhit_2)) (* (* _index_2 25) (LocalVariables|GetActorForwardVector))) "0.000000,0.000000,100.000000") "TraceTypeQuery1" false 0 "None"))
                          (if _returnvalue_3
                            (Utilities|FlowControl|Sequence
                              (:then_0
                                (goto _label_2 Break))
                              (:then_1
                                (LocalVariables|SetMantleEnd (.impactpoint _outhit_3))
                                ;[1 1 1] can jump on?
                                (bind _index_3 (Utilities|FlowControl|ForLoopwithBreak 1 4)
                                  (:LoopBody
                                    (bind _returnvalue_4 (Collision|SphereTraceByChannel (Math|Vector|MakeVector (.x (+ (LocalVariables|GetMantleStartPosition) (Math|Vector|MakeVector 0.0 0.0 (+ (* _index_3 35) 15.0)))) (.y (+ (LocalVariables|GetMantleStartPosition) (Math|Vector|MakeVector 0.0 0.0 (+ (* _index_3 35) 15.0)))) (.z (+ (LocalVariables|GetMantleStartPosition) (Math|Vector|MakeVector 0.0 0.0 (+ (* _index_3 35) 15.0))))) (Math|Vector|MakeVector (.x (LocalVariables|GetMantleEnd)) (.y (LocalVariables|GetMantleEnd)) (.z (+ (LocalVariables|GetMantleStartPosition) (Math|Vector|MakeVector 0.0 0.0 (+ (* _index_3 35) 15.0))))) 3e+01 "TraceTypeQuery1" false 0 "None" true "(R=1.000000,G=0.680251,B=0.000000,A=1.000000)" "(R=0.000000,G=0.971714,B=1.000000,A=1.000000)"))
                                    (if _returnvalue_4
                                      (return false 0)))
                                  (:Completed
                                    (return true (Utilities|Array|MakeArray (Utilities|Struct|MakePMC_WarpPoint "MantleStart" (LocalVariables|GetMantleStartPosition) (LocalVariables|GetMantleStartAngle)) (Utilities|Struct|MakePMC_WarpPoint "MantleEnd" (LocalVariables|GetMantleEnd) "0.000000,0.000000,0.000000"))))))))))
                      (else
                        (return false 0)))))))
            (:Completed
              (return false 0))))))
    (:Is%20Not%20Valid
      (return false 0))))

(fn GetClimbPosition
  (Utilities|IsValid (Variables|Default|GetOwner)
    (:Is%20Valid
      (Utilities|FlowControl|Sequence
        (:then_0
          (LocalVariables|SetActorForwardVector (Transformation|GetActorForwardVector (Variables|Default|GetOwner))))
        (:then_1
          (LocalVariables|SetActorLocation (Transformation|GetActorLocation (Variables|Default|GetOwner))))
        (:then_2
          ;[1 1 1] Seatching For an obsticle to climb
          (bind _index (Utilities|FlowControl|ForLoopwithBreak 1 3 :!label _label)
            (:LoopBody
              (bind (_outhit _returnvalue) (Collision|SphereTraceByChannel (+ (LocalVariables|GetActorLocation) (Math|Vector|MakeVector 0.0 0.0 (* _index 40))) (+ (+ (LocalVariables|GetActorLocation) (Math|Vector|MakeVector 0.0 0.0 (* _index 40))) (* (LocalVariables|GetActorForwardVector) 5e+01)) 5.0 "TraceTypeQuery1" false 0 "None" true "(R=1.000000,G=0.680251,B=0.000000,A=1.000000)" "(R=0.000000,G=0.971714,B=1.000000,A=1.000000)"))
              (if _returnvalue
                (Utilities|FlowControl|Sequence
                  (:then_0
                    (goto _label Break))
                  (:then_1
                    ;[1 1 1] Getting vault points
                    (LocalVariables|SetClimbStartRot (Math|Rotator|MakeRotfromX (* (.ImpactNormal (Collision|BreakHitResult _outhit)) -1.0)))
                    (bind _index_2 (Utilities|FlowControl|ForLoopwithBreak 0 5 :!label _label_2)
                      (:LoopBody
                        (bind (_outhit_2 _returnvalue_2) (Collision|SphereTraceByChannel (+ (* (* _index_2 50) (LocalVariables|GetActorForwardVector)) (+ (.ImpactPoint (Collision|BreakHitResult _outhit)) "0.000000,0.000000,75.000000")) (- (+ (* (* _index_2 50) (LocalVariables|GetActorForwardVector)) (+ (.ImpactPoint (Collision|BreakHitResult _outhit)) "0.000000,0.000000,75.000000")) "0.000000,0.000000,130.000000") 1e+01 "TraceTypeQuery1" false 0 "None" true "(R=0.125059,G=0.000000,B=1.000000,A=1.000000)" "(R=1.000000,G=0.856791,B=0.000000,A=1.000000)"))
                        (if _returnvalue_2
                          (if (== _index_2 0)
                            (bind _output_get (LocalVariables|SetClimbStartCollisionEdge (.ImpactPoint (Collision|BreakHitResult _outhit_2))))
                            (LocalVariables|SetClimbStartPosition (- _output_get (* (LocalVariables|GetActorForwardVector) 1e+01)))
                            (Utilities|FlowControl|Sequence
                              (:then_0
                                (goto _label_2 Break))
                              (:then_1
                                ;[0.15 0.15 0.15 0.5] EndPosition
                                (bind _index_3 (Utilities|FlowControl|ForLoopwithBreak 1 3 :!label _label_3)
                                  (:LoopBody
                                    (bind (_outhit_3 _returnvalue_3) (Collision|SphereTraceByChannel (+ (LocalVariables|GetClimbStartCollisionEdge) (* (LocalVariables|GetActorForwardVector) (+ _index_3 5))) (- (+ (LocalVariables|GetClimbStartCollisionEdge) (* (LocalVariables|GetActorForwardVector) (+ _index_3 5))) "0.000000,0.000000,40.000000") 5.0 "TraceTypeQuery1" false 0 "None" true "(R=1.000000,G=0.000000,B=0.725684,A=1.000000)" "(R=1.000000,G=0.810927,B=0.000000,A=1.000000)"))
                                    (if _returnvalue_3
                                      (LocalVariables|SetClimbEndPosition (+ (.location _outhit_3) (* (LocalVariables|GetActorForwardVector) 1e+01)))
                                      ;[1 1 1] can stand?
                                      (bind _index_4 (Utilities|FlowControl|ForLoopwithBreak 0 3)
                                        (:LoopBody
                                          (bind _returnvalue_4 (Collision|SphereTraceByChannel (Math|Vector|MakeVector (.x (+ (LocalVariables|GetClimbStartCollisionEdge) (Math|Vector|MakeVector 0.0 0.0 (+ (* _index_4 55) 5.0)))) (.y (+ (LocalVariables|GetClimbStartCollisionEdge) (Math|Vector|MakeVector 0.0 0.0 (+ (* _index_4 55) 5.0)))) (.z (+ (LocalVariables|GetClimbStartCollisionEdge) (Math|Vector|MakeVector 0.0 0.0 (+ (* _index_4 55) 5.0))))) (Math|Vector|MakeVector (.x (+ (LocalVariables|GetClimbEndPosition) (* (LocalVariables|GetActorForwardVector) 3e+01))) (.y (+ (LocalVariables|GetClimbEndPosition) (* (LocalVariables|GetActorForwardVector) 3e+01))) (.z (+ (LocalVariables|GetClimbStartCollisionEdge) (Math|Vector|MakeVector 0.0 0.0 (+ (* _index_4 55) 5.0))))) 1.0 "TraceTypeQuery1" false 0 "None" true "(R=1.000000,G=0.000000,B=0.715927,A=1.000000)" "(R=0.000000,G=1.000000,B=0.148498,A=1.000000)"))
                                          (if _returnvalue_4
                                            (return false 0)))
                                        (:Completed
                                          (return true (Utilities|Array|MakeArray (Utilities|Struct|MakePMC_WarpPoint "ClimbStart" (LocalVariables|GetClimbStartPosition) (LocalVariables|GetClimbStartRot)) (Utilities|Struct|MakePMC_WarpPoint "ClimbEnd" (LocalVariables|GetClimbEndPosition) "0.000000,0.000000,0.000000")))))
                                      (else
                                        (goto _label_3 Break))))
                                  (:Completed
                                    (return false 0)))))))))))))
            (:Completed
              (return false 0))))))
    (:Is%20Not%20Valid
      (return false 0))))

(fn SetVaultMotionWarp
  (params (Points :type Array%20of%20PMC%20Warp%20Point%20Structures))
  (bind _motionwarpingcomponent (PrivateGetters|GetMotionWarpingComponent))
  (Utilities|IsValid _motionwarpingcomponent
    (:Is%20Valid
      (for _array_element Points
        (Class|MotionWarpingComponent|AddorUpdateWarpTarget _motionwarpingcomponent (Utilities|Struct|MakeMotionWarpingTarget (.warppointname _array_element) (.position _array_element) (.rotation _array_element) 0 "None" false "TargetsForwardVector" "0.000000,0.000000,0.000000" "0.000000,0.000000,0.000000" 0))))))

(fn Parkour
  (bind _canclimb (CallFunction|GetCanClimb))
  (if _canclimb
    (bind (_can_climb _warp_points) (PrivateParkour|GetClimbPosition))
    (if _can_climb
      (CallFunction|StartParkourVault _warp_points (Variables|Default|GetClimbAnimMontage))
      (return true)
      (else
        _)))
  (bind _canvault (CallFunction|GetCanVault))
  (if _canvault
    (bind (_can_mantle _warp_points_2) (PrivateParkour|GetMantlePosition))
    (if _can_mantle
      (CallFunction|StartParkourVault _warp_points_2 (Variables|Default|GetMantleAnimMontage))
      (return true)
      (else
        (bind (_can_vault _warp_points_3) (PrivateParkour|GetVaultOverPosition))
        (if _can_vault
          (CallFunction|StartParkourVault _warp_points_3 (Variables|Default|GetVaultAnimMontage))
          (return true)
          (else
            (return false)))))
    (else
      (return false))))

(fn StartParkour
  (bind _charactermovementcomponent (PrivateGetters|GetCharacterMovementComponent))
  (Pawn|Components|CharacterMovement|SetMovementMode _charactermovementcomponent "MOVE_Flying" 0)
  (Collision|SetActorEnableCollision (Variables|Default|GetOwner) false)
  (Default|CallOnParkour))