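; Actor component that manages a character's integer stamina, firing events on change, empty and full.
; Continuous drain and passive restore run as mutually exclusive, self-calling delay loops; one-off drains can schedule restore through a retriggerable-delay debounce.
; Emptying stamina stops draining and starts a cooldown that fails action checks, and restoring from empty waits an extra delay.
; The action check ignores its cost, testing only cooldown and non-negative stamina.
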(event Custom|StaminaDrainTick
  ;[0.15 0.15 0.15 0.5] Continious Drain
  (if (Variables|StaminaSystem|GetIsStaminaDraining)
    (StaminaSystem|DrainStamina (Variables|StaminaSystem|GetPassiveDrainAmount) false)
    (Utilities|FlowControl|Delay (Variables|StaminaSystem|GetStaminaDrainSpeed))
    (CallFunction|StaminaDrainTick)))

(event Custom|StaminaRestoreTick
  ;[0.15 0.15 0.15 0.5] Passive restore
  (if (Variables|StaminaSystem|GetIsStaminaRestoring)
    (if (<= (Variables|StaminaSystem|GetCurrentStamina) 0)
      (Utilities|FlowControl|RetriggerableDelay (Variables|StaminaSystem|GetFullDrainRestoreCooldownTime)))
    (StaminaSystem|RestoreStamina (Variables|StaminaSystem|GetPassiveRestoreAmount))
    (Utilities|FlowControl|Delay (Variables|StaminaSystem|GetStaminaRestoreSpeed))
    (CallFunction|StaminaRestoreTick)))

(event Custom|StaminaDrainCoolDown
  ;[0.15 0.15 0.15 0.5] Post full drain cooldown reset
  (Variables|StaminaSystem|SetIsPostDrainedCooldown true)
  (Utilities|FlowControl|Delay (Variables|StaminaSystem|GetPostDrainCooldownTime))
  (Variables|StaminaSystem|SetIsPostDrainedCooldown false))

(event Custom|SchedulePassiveStaminaRestoreEvent
  ;[0.15 0.15 0.15 0.5] Passive restore schedule debounce
  (Utilities|FlowControl|RetriggerableDelay (Variables|StaminaSystem|GetPassiveRestoreDebounceTime))
  (if (not (Variables|StaminaSystem|GetIsStaminaRestoring))
    (StaminaSystem|StartPassiveStaminaRestore)))

(event EventBeginPlay
  (Private|InitStamina))

(event EventTick
  (params (DeltaSeconds :type Float%20%28single-precision%29)))

(fn SetStamina
  (params (Value :type Integer))
  (bind _output_get (Variables|StaminaSystem|SetCurrentStamina (Math|Integer|Clamp(Integer) Value 0 (Variables|StaminaSystem|GetMaxStamina))))
  (Default|CallOnStaminaChange _output_get)
  (return (Variables|StaminaSystem|GetCurrentStamina)))

(fn InitStamina
  (if (== (Variables|StaminaSystem|GetCurrentStamina) -1)
    (Variables|StaminaSystem|SetCurrentStamina (Variables|StaminaSystem|GetMaxStamina))))

(fn StartStaminaDrain
  (params (DrainValue :type Integer))
  (Variables|StaminaSystem|SetPassiveDrainAmount DrainValue)
  (StaminaSystem|StopPassiveStaminaRestore)
  (if (not (Variables|StaminaSystem|GetIsStaminaDraining))
    (Variables|StaminaSystem|SetIsStaminaDraining true)
    (CallFunction|StaminaDrainTick)))

(fn StopStaminaDrain
  (Variables|StaminaSystem|SetIsStaminaDraining false))

(fn DrainStamina
  (params (DrainAmount :type Integer) (IsAutoRestore :type Boolean))
  (LocalVariables|SetLocalShouldRestore IsAutoRestore)
  (bind _new_stamina (Private|SetStamina (- (Variables|StaminaSystem|GetCurrentStamina) DrainAmount)))
  (StaminaSystem|StopPassiveStaminaRestore)
  (if (LocalVariables|GetLocalShouldRestore)
    (CallFunction|SchedulePassiveStaminaRestoreEvent))
  ;[0.15 0.15 0.15 0.5] Set cooldown on fully drained stamina
  (if (<= _new_stamina 0)
    (Default|CallOnOutOfStamina)
    (StaminaSystem|StopStaminaDrain)
    (CallFunction|StaminaDrainCoolDown))
  (return _new_stamina))

(fn StartPassiveStaminaRestore
  (StaminaSystem|StopStaminaDrain)
  (if (not (Variables|StaminaSystem|GetIsStaminaRestoring))
    (Variables|StaminaSystem|SetIsStaminaRestoring true)
    (CallFunction|StaminaRestoreTick)))

(fn StopPassiveStaminaRestore
  (Variables|StaminaSystem|SetIsStaminaRestoring false))

(fn GetHasEnoughStaminaforAction
  (params (ActionCost :type Integer))
  (if (Variables|StaminaSystem|GetIsPostDrainedCooldown)
    (return false)
    (else
      (return (>= (Variables|StaminaSystem|GetCurrentStamina) 0)))))

(fn RestoreStamina
  (params (Restore%20Amount :type Integer))
  (bind _new_stamina (Private|SetStamina (+ Restore%20Amount (Variables|StaminaSystem|GetCurrentStamina))))
  (if (== _new_stamina (Variables|StaminaSystem|GetMaxStamina))
    (Default|CallOnFullStamina)
    (StaminaSystem|StopPassiveStaminaRestore))
  (return (Variables|StaminaSystem|GetCurrentStamina)))