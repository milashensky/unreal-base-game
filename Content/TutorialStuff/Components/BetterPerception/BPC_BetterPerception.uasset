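; AI Controller component that turns perception updates into aggression-based target selection and team coordination.
; A per-actor aggression map, fed by sightings, damage and teammate reports, picks targets, with a close-range override and memory of the last target.
; Teammates found through BPI_AITeamMember exchange spotted, lost, target and death messages, some with sound cues.
; Shared locations blend last sensed and actual positions; unseen reported targets raise an investigate event instead of being selected.
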(event Custom|OnPerceptionUpdated_Event
  (params (UpdatedActors :type Array%20of%20Actor%20Object%20References))
  (baseperception|HandlePerceptionUpdate UpdatedActors))

(event Custom|TargetUpdateTick
  ;[0.15 0.15 0.15 0.5] Sends updates to teammates while target is selected
  (Utilities|FlowControl|RetriggerableDelay 3.0)
  (Utilities|IsValid (Variables|Default|GetCurrentTarget)
    (:Is%20Valid
      (TeamCommunicationPrivate|SendTargetSelected (Variables|Default|GetCurrentTarget))
      (CallFunction|TargetUpdateTick))))

(event Custom|AggressionUpdateTick
  (bind _aicontroller (Variables|Default|GetAIController))
  (bind _returnvalue (Pawn|GetControlledPawn _aicontroller))
  ;[0.15 0.15 0.15 0.5] Increases Aggression To percieved enemies, while decreasing it to lost enemies
  (Utilities|IsValid _aicontroller
    (:Is%20Valid
      (Utilities|IsValid _returnvalue
        (:Is%20Valid
          (bind _isdead (Class|PBIDamageable|GetIsDead(Message) _returnvalue))
          (if _isdead
            (Attack/aggression|UpdateAggressionValues)
            (Utilities|FlowControl|RetriggerableDelay 1.0)
            (CallFunction|AggressionUpdateTick)))))))

(event Custom|ForgetTargetTick
  ;[0.15 0.15 0.15 0.5] Helps to keep the memory of last target, so AI doens't switch right away if not interested. but if dead, forget right away
  (Utilities|IsValid (Variables|Default|GetLastTarget)
    (:Is%20Valid
      (bind _isdead (Class|PBIDamageable|GetIsDead(Message) (Variables|Default|GetLastTarget)))
      (if _isdead
        (Variables|Default|SetLastTarget 0)
        (else
          (Utilities|FlowControl|RetriggerableDelay (/ (.Value (Utilities|Map|Find (Variables|Default|GetAggressionByActor) (Variables|Default|GetLastTarget))) 1e+01))
          (Utilities|IsValid (Variables|Default|GetCurrentTarget)
            (:Is%20Not%20Valid
              (Variables|Default|SetLastTarget 0)
              (Attack/aggression|ClearTarget))))))))

(event EventBeginPlay
  ;[0.15 0.15 0.15 0.5] Init
  (bind _asaicontroller (Utilities|Casting|CastToAIController (Components|GetOwner)))
  (Variables|Default|SetAIController _asaicontroller)
  (Utilities|FlowControl|Sequence
    (:then_0
      (bind _teamid (Class|BPITeamMember|GetTeamId(Message) (Variables|Default|GetAIController)))
      (Variables|Default|SetTeamId _teamid))
    (:then_1
      (Variables|Default|SetAIPerceptionComponent (Class|AIController|GetAIPerceptionComponent (Variables|Default|GetAIController))))
    (:then_2
      (EventDispatchers|AssignOnPerceptionUpdated (Variables|Default|GetAIPerceptionComponent) (delegate Custom|OnPerceptionUpdated_Event)))
    (:then_4
      (CallFunction|AggressionUpdateTick))))

(fn CompareDistance
  (params (CurrentTarget :type Actor%20Object%20Reference) (NewTarget :type Actor%20Object%20Reference))
  (bind _aicontroller (Variables|Default|GetAIController))
  (bind _returnvalue (Pawn|GetControlledPawn _aicontroller))
  ;[0.15 0.15 0.15 0.5] helps to force engage with a closeup enemy
  (Utilities|IsValid _aicontroller
    (:Is%20Valid
      (Utilities|IsValid _returnvalue
        (:Is%20Valid
          (LocalVariables|SetControlledPawn _returnvalue)
          (if (< (Transformation|GetDistanceTo (LocalVariables|GetControlledPawn) CurrentTarget) 4e+02)
            (return false)
            (else
              (return (< (Transformation|GetDistanceTo (LocalVariables|GetControlledPawn) NewTarget) 2e+02)))))))))

(fn EvaluateasTarget
  (params (PossibleTarget :type Actor%20Object%20Reference))
  (bind _aggressionbyactor (Variables|Default|GetAggressionByActor))
  (bind (_value _returnvalue) (Utilities|Map|Find _aggressionbyactor PossibleTarget))
  (bind _isaggressive (Attack/aggression|GetDefaultAggressiontoActor PossibleTarget))
  (if _isaggressive
    (LocalVariables|SetActorAggression _value)
    (if _returnvalue
      (Utilities|IsValid (Variables|Default|GetCurrentTarget)
        (:Is%20Valid
          ;[0.15 0.15 0.15 0.5] Prioritize new one, if breathes down the neck
          (bind _isbettertarget (Attack/aggression|CompareDistance (Variables|Default|GetCurrentTarget) PossibleTarget))
          (if _isbettertarget
            (return true)
            (else
              (return (> (LocalVariables|GetActorAggression) (.Value (Utilities|Map|Find (Variables|Default|GetAggressionByActor) (Variables|Default|GetCurrentTarget))))))))
        (:Is%20Not%20Valid
          (Utilities|IsValid (Variables|Default|GetLastTarget)
            (:Is%20Valid
              ;[0.15 0.15 0.15 0.5] Prioritize new one, if breathes down the neck
              (bind _isbettertarget_2 (Attack/aggression|CompareDistance (Variables|Default|GetLastTarget) PossibleTarget))
              (if _isbettertarget_2
                (return true)
                (else
                  ;[0.15 0.15 0.15 0.5] Helps to keep track of a "really annoing" target
                  (return (> (* (LocalVariables|GetActorAggression) 3.0) (.Value (Utilities|Map|Find (Variables|Default|GetAggressionByActor) (Variables|Default|GetLastTarget))))))))
            (:Is%20Not%20Valid
              (return true)))))
      (else
        (return false)))
    (else
      (return false))))

(fn OnTargetDeath
  (params (Damage :type S%20Damage%20Info%20Structure))
  (Utilities|FlowControl|Sequence
    (:then_0
      (if (== (Variables|Default|GetCurrentTarget) (Variables|Default|GetLastTarget))
        (Variables|Default|SetLastTarget 0)))
    (:then_1
      (Attack/aggression|ClearTarget))))

(fn DefineAggressionValue
  (params (Actor :type Actor%20Object%20Reference))
  (if (Utilities|Map|Contains (Variables|Default|GetAggressionByActor) Actor)
    (return)
    (else
      (bind (_aggression _isaggressive) (Attack/aggression|GetDefaultAggressiontoActor Actor))
      (if _isaggressive
        (Utilities|Map|Add (Variables|Default|GetAggressionByActor) Actor _aggression)))))

(fn GetDefaultAggressiontoActor
  (params (Actor :type Actor%20Object%20Reference))
  (Utilities|IsValid Actor
    (:Is%20Valid
      (bind _isdamageable (Class|PBIDamageable|IsDamageable(Message) Actor))
      (if (and _isdamageable (not (Actor|ActorHasTag Actor "Ignore")))
        (bind _isdead (Class|PBIDamageable|GetIsDead(Message) Actor))
        (if _isdead
          (return 0.0 false)
          (else
            (bind _teamid (Class|BPITeamMember|GetTeamId(Message) Actor))
            (if (== _teamid (Variables|Default|GetTeamId))
              (return 0.0 false)
              (else
                (return 1.0 true)))))))))

(fn UpdateAggressionValues
  (bind (_keypin _valuepin) (Utilities|Map|ForEachLoop(Map) (Variables|Default|GetAggressionByActor))
    (:then
      (Attack/aggression|UpdateActorAggression _keypin _valuepin))))

(fn UpdateActorAggression
  (params (ActorKey :type Actor%20Object%20Reference) (CurrentAggression :type Float%20%28double-precision%29))
  (bind _aggression (Attack/aggression|GetDefaultAggressiontoActor ActorKey))
  (LocalVariables|SetDefaultAggression _aggression)
  (bind _iscurrentlyperceived (BasePerception|GetIsActorPerceved ActorKey))
  ;[0.15 0.15 0.15 0.5] Cooling down if actor is not seen, and gaining aggression if seen.
  ; TODO: dynamic values
  (if _iscurrentlyperceived
    (LocalVariables|SetIncrementValue 0.5)
    (else
      (LocalVariables|SetIncrementValue -0.5)))
  ;[0.15 0.15 0.15 0.5] don't go above or below the base value during tick, only manually
  (if (>= CurrentAggression (LocalVariables|GetDefaultAggression))
    (Attack/aggression|AddActorAggression ActorKey (LocalVariables|GetIncrementValue))))

(fn AddActorAggression
  (params (Actor :type Actor%20Object%20Reference) (AggressionIncrement :type Float%20%28double-precision%29))
  (bind _aggressionbyactor (Variables|Default|GetAggressionByActor))
  (bind (_value _returnvalue) (Utilities|Map|Find _aggressionbyactor Actor))
  (bind (_aggression _isaggressive) (Attack/aggression|GetDefaultAggressiontoActor Actor))
  (if _isaggressive
    (if _returnvalue
      (LocalVariables|SetCurrentAggression _value)
      (else
        (LocalVariables|SetCurrentAggression _aggression)))
    (Utilities|Map|Add (Variables|Default|GetAggressionByActor) Actor (+ (LocalVariables|GetCurrentAggression) AggressionIncrement))))

(fn SetTarget
  (params (TargetActor :type Actor%20Object%20Reference))
  (if (!= TargetActor (Variables|Default|GetCurrentTarget))
    (Utilities|FlowControl|Sequence
      (:then_0
        (bind _output_get (Variables|Default|SetCurrentTarget TargetActor))
        (Variables|Default|SetLastTarget _output_get)
        ;[0.15 0.15 0.15 0.5] Not really needed, but will reset the timer
        (CallFunction|ForgetTargetTick))
      (:then_1
        (Attack/aggression|AddActorAggression TargetActor 0.3))
      (:then_2
        (TeamCommunicationPrivate|SendTargetSelected TargetActor))
      (:then_3
        (bind _healthcomponent (Class|PBIDamageable|GetHealthComponent(Message) TargetActor))
        (Utilities|IsValid _healthcomponent
          (:Is%20Valid
            (EventDispatchers|BindEventtoOnDeath _healthcomponent (EventDispatchers|CreateEvent :!event OnTargetDeath)))))
      (:then_4
        (Default|CallOnTargetSelected TargetActor))
      (:then_5
        (CallFunction|TargetUpdateTick)))))

(fn ClearTarget
  (Utilities|FlowControl|Sequence
    (:then_0
      (Utilities|IsValid (Variables|Default|GetCurrentTarget)
        (:Is%20Valid
          (bind _healthcomponent (Class|PBIDamageable|GetHealthComponent(Message) (Variables|Default|GetCurrentTarget)))
          (Utilities|IsValid _healthcomponent
            (:Is%20Valid
              (EventDispatchers|UnbindEventfromOnDeath _healthcomponent (EventDispatchers|CreateEvent :!event OnTargetDeath)))))))
    (:then_1
      (Utilities|IsValid (Variables|Default|GetCurrentTarget)
        (:Is%20Valid
          (TeamCommunicationPrivate|SendTargetLost (Variables|Default|GetCurrentTarget)))))
    (:then_2
      (Variables|Default|SetCurrentTarget 0))
    (:then_3
      (CallFunction|ForgetTargetTick))
    (:then_4
      (Default|CallOnTargetLost))
    (:then_5
      (baseperception|HandlePerceptionUpdate (Class|AIPerceptionComponent|GetCurrentlyPerceivedActors (Variables|Default|GetAIPerceptionComponent))))))

(fn GetLastSensedLocation
  (params (Actor :type Actor%20Object%20Reference))
  (bind (_info _returnvalue) (Class|AIPerceptionComponent|GetActorsPerception (Variables|Default|GetAIPerceptionComponent) Actor))
  (if _returnvalue
    (for _array_element (.lastsensedstimuli _info)
      (if (or (< (.age _array_element) (LocalVariables|GetLastSensedAge)) (< (LocalVariables|GetLastSensedAge) 0.0))
        (LocalVariables|SetLastSensedLocation (.stimuluslocation _array_element))
        (LocalVariables|SetLastSensedAge (.age _array_element))
        (LocalVariables|SetIsFound true)))
    (return (LocalVariables|GetLastSensedLocation) (LocalVariables|GetIsFound))
    (else
      (return "0, 0, 0" false))))

(fn CheckIsActorPercieved
  (params (ActorPerceptionBlueprintInfo :type Actor%20Perception%20Blueprint%20Info%20Structure%20%28by%20ref%29))
  (for _array_element (.LastSensedStimuli (Utilities|Struct|BreakActorPerceptionBlueprintInfo ActorPerceptionBlueprintInfo))
    (if (.bsuccessfullysensed _array_element)
      (return true)))
  (return false))

(fn HandlePerceptionUpdate
  (params (UpdatedActors :type Array%20of%20Actor%20Object%20References))
  (for _array_element UpdatedActors
    (baseperception|SenceActor _array_element)))

(fn UpdatePercevedActor
  (params (ActorPerceptionBlueprintInfo :type Actor%20Perception%20Blueprint%20Info%20Structure%20%28by%20ref%29))
  (bind (_target _lastsensedstimuli) (Utilities|Struct|BreakActorPerceptionBlueprintInfo ActorPerceptionBlueprintInfo))
  (LocalVariables|SetPercievedActor _target)
  (LocalVariables|SetLastStimulus (Utilities|Array|Get(acopy) _lastsensedstimuli (Utilities|Array|LastIndex _lastsensedstimuli)))
  (Utilities|FlowControl|Sequence
    (:then_0
      (Attack/aggression|DefineAggressionValue (LocalVariables|GetPercievedActor)))
    (:then_1
      (if (.bsuccessfullysensed (LocalVariables|GetLastStimulus))
        (bind _returnvalue (Class|AIPerceptionSystem|GetSenseClassforStimulus (LocalVariables|GetLastStimulus)))
        (if (== _returnvalue "/Script/AIModule.AISense_Damage")
          (Attack/aggression|AddActorAggression (LocalVariables|GetPercievedActor) 1e+01))))
    (:then_2
      (TeamCommunicationPrivate|SendActorSpotted (LocalVariables|GetPercievedActor)))
    (:then_3
      (bind _istarget (Attack/aggression|EvaluateasTarget (LocalVariables|GetPercievedActor)))
      (if _istarget
        (Attack/aggression|SetTarget (LocalVariables|GetPercievedActor))))))

(fn SenceActor
  (params (Actor :type Actor%20Object%20Reference))
  (bind _info (Class|AIPerceptionComponent|GetActorsPerception (Variables|Default|GetAIPerceptionComponent) Actor))
  (bind _ispercieved (baseperception|CheckIsActorPercieved _info))
  (if _ispercieved
    (baseperception|UpdatePercevedActor _info)
    (else
      (baseperception|ActorLost Actor))))

(fn ActorLost
  (params (Lost%20Actor :type Actor%20Object%20Reference))
  (bind _currenttarget (Variables|Default|GetCurrentTarget))
  (TeamCommunicationPrivate|SendActorForgotten Lost%20Actor)
  (Utilities|IsValid _currenttarget
    (:Is%20Valid
      (if (== _currenttarget Lost%20Actor)
        (Attack/aggression|ClearTarget)))))

(fn ReceiveTargetSelected
  (params (TargetActor :type Actor%20Object%20Reference) (Last%20known%20location :type Vector))
  (Utilities|FlowControl|Sequence
    (:then_0
      ;[0.15 0.15 0.15 0.5] Add common cause, and get actor known
      (Attack/aggression|AddActorAggression TargetActor 0.05))
    (:then_1
      (bind _istarget (Attack/aggression|EvaluateasTarget TargetActor))
      (if _istarget
        (bind _iscurrentlyperceived (BasePerception|GetIsActorPerceved TargetActor))
        (if _iscurrentlyperceived
          (Attack/aggression|SetTarget TargetActor)
          (else
            (Default|CallOnTargetLocationInvestigate Last%20known%20location)))))
    (:then_2
      (return true))))

(fn ReceiveTargetLost
  (params (TargetActor :type Actor%20Object%20Reference))
  (bind _currenttarget (Variables|Default|GetCurrentTarget))
  (Utilities|FlowControl|Sequence
    (:then_0
      (Utilities|IsValid _currenttarget
        (:Is%20Valid
          (TeamCommunicationPrivate|SendTargetSelected _currenttarget))))
    (:then_1
      (return true))))

(fn ReceiveActorSpotted
  (params (TargetActor :type Actor%20Object%20Reference) (Last%20known%20location :type Vector))
  (return true))

(fn ReceiveActorForgotten
  (params (TargetActor :type Actor%20Object%20Reference))
  (return true))

(fn GetCommunicationUsableActorLocation
  (params (Actor :type Actor%20Object%20Reference))
  (Utilities|FlowControl|Sequence
    (:then_0
      (bind (_lastlocation _issuccessful) (baseperception|GetLastSensedLocation Actor))
      (if _issuccessful
        (LocalVariables|SetLastLocation _lastlocation)
        (else
          (LocalVariables|SetLastLocation (Transformation|GetActorLocation (Variables|Default|GetAIController))))))
    (:then_1
      ;[0.15 0.15 0.15 0.5] Return approximate direction, or a last point if known for sure
      (return (Math|Vector|Lerp(Vector) (LocalVariables|GetLastLocation) (Transformation|GetActorLocation Actor) 0.4)))))

(fn SendTargetSelected
  (params (Target%20Actor :type Actor%20Object%20Reference))
  (bind _location (TeamCommunicationPrivate|GetCommunicationUsableActorLocation Target%20Actor))
  (LocalVariables|SetLast%20known%20location _location)
  (bind _team_members (TeamCommunicationPrivate|GetCommunicationReceivers))
  (for _array_element _team_members
    (Class|BPIAITeamMember|ReceiveTargetSelected(Message) _array_element Target%20Actor (LocalVariables|GetLast%20known%20location))
    (CallFunction|PlayCommunicationSound (Variables|Sounds|GetCommunicateTargetSound))))

(fn SendTargetLost
  (params (Target%20Actor :type Actor%20Object%20Reference))
  (bind _team_members (TeamCommunicationPrivate|GetCommunicationReceivers))
  (for _array_element _team_members
    (Class|BPIAITeamMember|ReceiveTargetLost(Message) _array_element Target%20Actor)))

(fn SendActorSpotted
  (params (Actor :type Actor%20Object%20Reference))
  (Utilities|FlowControl|Sequence
    (:then_0
      (bind _location (TeamCommunicationPrivate|GetCommunicationUsableActorLocation Actor))
      (LocalVariables|SetLastKnownLocation _location))
    (:then_1
      (bind _team_members (TeamCommunicationPrivate|GetCommunicationReceivers))
      (for _array_element _team_members
        (Class|BPIAITeamMember|ReceiveActorSpotted(Message) _array_element Actor (LocalVariables|GetLastKnownLocation))))))

(fn SendActorForgotten
  (params (Actor :type Actor%20Object%20Reference))
  (bind _team_members (TeamCommunicationPrivate|GetCommunicationReceivers))
  (for _array_element _team_members
    (Class|BPIAITeamMember|ReceiveActorForgoten(Message) _array_element Actor)))

(fn GetCommunicationReceivers
  (bind _outactors (Actor|GetAllActorswithInterface "/Game/TutorialStuff/AI/Controllers/BPI_AITeamMember.BPI_AITeamMember_C"))
  (for _array_element _outactors
    (LocalVariables|SetIterActor _array_element)
    (if (not (== (Variables|Default|GetAIController) (LocalVariables|GetIterActor)))
      (bind _teamid (Class|BPITeamMember|GetTeamId(Message) (LocalVariables|GetIterActor)))
      (if (== _teamid (Variables|Default|GetTeamId))
        (Utilities|Array|Add (LocalVariables|GetFoundTeamMembers) (LocalVariables|GetIterActor)))))
  (return (LocalVariables|GetFoundTeamMembers)))

(fn SendTargetRequest
  (Utilities|FlowControl|Sequence
    (:then_0
      (Utilities|IsValid (Variables|Default|GetCurrentTarget)
        (:Is%20Valid
          (Default|CallOnTargetSelected (Variables|Default|GetCurrentTarget)))
        (:Is%20Not%20Valid
          (bind _team_members (TeamCommunicationPrivate|GetCommunicationReceivers))
          (for _array_element _team_members
            (Class|BPIAITeamMember|ReceiveTargetRequest(Message) _array_element)
            (CallFunction|PlayCommunicationSound (Variables|Sounds|GetRequestTargetSound))))))
    (:then_1
      (return true))))

(fn ReceiveTargetRequest
  (Utilities|FlowControl|Sequence
    (:then_0
      (Utilities|IsValid (Variables|Default|GetCurrentTarget)
        (:Is%20Valid
          (TeamCommunicationPrivate|SendTargetSelected (Variables|Default|GetCurrentTarget)))))
    (:then_1
      (return true))))

(fn SendTeammateDead
  (params (KilledBy :type Actor%20Object%20Reference))
  (Utilities|FlowControl|Sequence
    (:then_0
      (Utilities|IsValid KilledBy
        (:Is%20Valid
          (bind _team_members (TeamCommunicationPrivate|GetCommunicationReceivers))
          (for _array_element _team_members
            (Class|BPIAITeamMember|ReceiveTeammateDead(Message) _array_element KilledBy)))))
    (:then_1
      (return true))))

(fn ReceiveTeammateDead
  (params (KilledBy :type Actor%20Object%20Reference))
  (Utilities|IsValid KilledBy
    (:Is%20Valid
      (Attack/aggression|AddActorAggression KilledBy 5.0)
      (CallFunction|PlayCommunicationSound (Variables|Sounds|GetTeamMateDeadSound)))))

(fn GetIsActorPerceved
  (params (Actor :type Actor%20Object%20Reference))
  (return (Utilities|Array|ContainsItem (Class|AIPerceptionComponent|GetCurrentlyPerceivedActors (Variables|Default|GetAIPerceptionComponent)) Actor)))

(fn PlayCommunicationSound
  (params (Sound :type Sound%20Base%20Object%20Reference))
  (bind _aicontroller (Variables|Default|GetAIController))
  (bind _returnvalue (Pawn|GetControlledPawn _aicontroller))
  (Utilities|IsValid _aicontroller
    (:Is%20Valid
      (Utilities|IsValid _returnvalue
        (:Is%20Valid
          (Audio|PlaySoundatLocation Sound (Transformation|GetActorLocation _returnvalue) (Transformation|GetActorRotation _returnvalue) 1.0 1.0 0.0 0 0 _returnvalue 0))))))