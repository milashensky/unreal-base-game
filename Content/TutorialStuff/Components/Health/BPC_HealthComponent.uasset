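; Health component that tracks an actor's integer health and death state, handling damage and healing.
; BeginPlay fills CurrentHealth from MaxHealth when it holds the -1 sentinel, and SetHealth clamps every change and broadcasts it.
; TakeDamage reports a damage event, even for dead owners, then fires either damage-taken or death through Die.
; Once IsDead is set, further damage and healing are ignored.
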(event EventBeginPlay
  (HealthComponent|InitHealth))

(event EventTick
  (params (DeltaSeconds :type Float%20%28single-precision%29)))

(fn Heal
  (params (Amount :type Integer))
  (if (Variables|HealthComponent|GetIsDead)
    (return 0)
    (else
      (bind _new_heath (HealthComponent|SetHealth (+ Amount (Variables|HealthComponent|GetCurrentHealth))))
      (return _new_heath))))

(fn InitHealth
  (if (== (Variables|HealthComponent|GetCurrentHealth) -1)
    (Variables|HealthComponent|SetCurrentHealth (Variables|HealthComponent|GetMaxHealth))))

(fn Die
  (params (Damage :type S%20Damage%20Info%20Structure))
  (Variables|HealthComponent|SetIsDead true)
  (Default|CallOnDeath Damage))

(fn SetHealth
  (params (Value :type Integer))
  (bind _output_get (Variables|HealthComponent|SetCurrentHealth (Math|Integer|Clamp(Integer) Value 0 (Variables|HealthComponent|GetMaxHealth))))
  (Default|CallOnHealthChange _output_get)
  (return (Variables|HealthComponent|GetCurrentHealth)))

(fn TakeDamage
  (params (Damage :type S%20Damage%20Info%20Structure))
  (bind (_damageamount _damagelocation _damagesource) (Utilities|Struct|BreakS_DamageInfo Damage))
  (Class|AISenseDamage|ReportDamageEvent (Components|GetOwner) _damagesource (Math|Conversions|ToFloat(Integer) _damageamount) _damagelocation "0, 0, 0" "None")
  (if (Variables|HealthComponent|GetIsDead)
    (return false)
    (else
      (bind _new_heath (HealthComponent|SetHealth (- (Variables|HealthComponent|GetCurrentHealth) _damageamount)))
      (if (<= _new_heath 0)
        (HealthComponent|Die Damage)
        (else
          (Default|CallOnDamageTaken Damage)))
      (return true))))