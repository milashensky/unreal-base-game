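; Target lock component for a Character that finds, holds and switches lockable targets for player or AI owners.
; A sphere trace picks the target nearest a forward cone's center, and box traces switch it sideways.
; Tick eases owner rotation, steers control rotation with clamped pitch and sets AI focus, using a temporary pawn for predicted locations.
; Lock ends on target death or when periodic range and line-of-sight checks fail.
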(event Custom|LockToPredictionLocation
  (params (PredictionLocation :type Vector) (MaxLife :type Float%20%28double-precision%29))
  (bind _output_get (Variables|TargetLockPrivate|SetPredictionLocation PredictionLocation))
  ;[0.15 0.15 0.15 0.5] UE doesn't allow to focus pitch on location, only on a PAWN (actors don't work). so we create a tmp pawn. rotation controlls destroy time
  (Variables|TargetLockPrivate|SetIsUsePrediction true)
  (bind _returnvalue (Game|SpawnActorfromClass "/Game/TutorialStuff/Components/TargetLockComponent/BP_TempFocusPawn.BP_TempFocusPawn_C" (Math|Transform|MakeTransform _output_get (Math|Rotator|MakeRotator MaxLife 0.0 0.0)) "Undefined" "MultiplyWithRoot" 0 0))
  (Variables|TargetLockPrivate|SetTempFocusPawn _returnvalue)
  (Utilities|FlowControl|RetriggerableDelay MaxLife)
  (Variables|TargetLockPrivate|SetIsUsePrediction false)
  (Variables|TargetLockPrivate|SetTempFocusPawn 0))

(event Custom|VisibilityCheckTick
  (bind _isvisible (TargetLockPrivate|CheckIsTargetVisible))
  (if _isvisible
    (Utilities|FlowControl|Delay 2.5)
    (CallFunction|VisibilityCheckTick)
    (else
      (TargetLockComponent|EndTargetLock))))

(event EventBeginPlay
  (bind _ascharacter (Utilities|Casting|CastToCharacter (Components|GetOwner)))
  (bind _output_get (Variables|Default|SetOwnerCharacter _ascharacter))
  (bind _movementcomponent (Class|BPIMovableCharacter|GetCharacterMovementComponent(Message) _output_get))
  (Utilities|IsValid _movementcomponent
    (:Is%20Valid
      (Variables|TargetLockPrivate|SetOriginal%20Orient%20Rotation%20To%20Movement (Variables|/Script/Engine.CharacterMovementComponent|GetbOrientRotationToMovement _movementcomponent)))))

(event EventTick
  (params (DeltaSeconds :type Float%20%28single-precision%29))
  (TargetLockPrivateMovement|UpdateLockTargetPosition))

(fn ToggleTargetLock
  (Utilities|IsValid (Variables|Default|GetLockTarget)
    (:Is%20Valid
      (TargetLockComponent|EndTargetLock))
    (:Is%20Not%20Valid
      (TargetLockComponent|StartTargetLock))))

(fn SetTargetLockActor
  (params (LockTarget :type Actor%20Object%20Reference))
  (TargetLockComponent|EndTargetLock)
  (Utilities|IsValid LockTarget
    (:Is%20Valid
      (Variables|Default|SetLockTarget LockTarget)
      (Utilities|FlowControl|Sequence
        (:then_0
          (bind _healthcomponent (Class|PBIDamageable|GetHealthComponent(Message) (Variables|Default|GetLockTarget)))
          (Utilities|IsValid _healthcomponent
            (:Is%20Valid
              (EventDispatchers|BindEventtoOnDeath _healthcomponent (EventDispatchers|CreateEvent :!event OnTargetDeath)))))
        (:then_1
          (bind _movementcomponent (Class|BPIMovableCharacter|GetCharacterMovementComponent(Message) (Variables|Default|GetOwnerCharacter)))
          (Utilities|IsValid _movementcomponent
            (:Is%20Valid
              (Variables|/Script/Engine.CharacterMovementComponent|SetbOrientRotationToMovement _movementcomponent false))))
        (:then_2
          (Default|CallOnTargetLocked (Variables|Default|GetLockTarget)))
        (:then_3
          (CallFunction|VisibilityCheckTick))))))

(fn EndTargetLock
  (Utilities|FlowControl|Sequence
    (:then_0
      (bind _healthcomponent (Class|PBIDamageable|GetHealthComponent(Message) (Variables|Default|GetLockTarget)))
      (Utilities|IsValid _healthcomponent
        (:Is%20Valid
          (EventDispatchers|UnbindEventfromOnDeath _healthcomponent (EventDispatchers|CreateEvent :!event OnTargetDeath)))))
    (:then_1
      (Default|CallOnTargetUnlocked (Variables|Default|GetLockTarget)))
    (:then_2
      (bind _movementcomponent (Class|BPIMovableCharacter|GetCharacterMovementComponent(Message) (Variables|Default|GetOwnerCharacter)))
      (Utilities|IsValid _movementcomponent
        (:Is%20Valid
          (Variables|/Script/Engine.CharacterMovementComponent|SetbOrientRotationToMovement _movementcomponent (Variables|TargetLockPrivate|GetOriginal%20Orient%20Rotation%20To%20Movement)))))
    (:then_3
      (Variables|Default|SetLockTarget 0))
    (:then_4
      (Utilities|IsValid (AI|GetAIController (Variables|Default|GetOwnerCharacter))))))

(fn GetTargetLockLocation
  (bind _locktarget (Variables|Default|GetLockTarget))
  (Utilities|IsValid (Variables|Default|GetLockTarget)
    (:Is%20Valid
      (if (Variables|TargetLockPrivate|GetIsUsePrediction)
        (return true (Variables|Default|GetLockTarget) (Variables|TargetLockPrivate|GetPredictionLocation))
        (else
          (return true _locktarget (Transformation|GetActorLocation _locktarget)))))
    (:Is%20Not%20Valid
      (return false 0 "0, 0, 0"))))

(fn SelectTargettoRight
  (bind _ownercharacter (Variables|Default|GetOwnerCharacter))
  (Utilities|IsValid _ownercharacter
    (:Is%20Valid
      (bind _ischanged (TargetLockPrivate|SelectTargetSide (Transformation|GetActorRightVector _ownercharacter)))
      (return _ischanged))))

(fn SelectTargettoLeft
  (bind _ownercharacter (Variables|Default|GetOwnerCharacter))
  (Utilities|IsValid _ownercharacter
    (:Is%20Valid
      (bind _ischanged (TargetLockPrivate|SelectTargetSide (* (Transformation|GetActorRightVector _ownercharacter) -1)))
      (return _ischanged))))

(fn StartTargetLock
  (bind (_istargetfound _besttarget) (TargetLockPrivateMovement|TraceTargetLockCone))
  (if _istargetfound
    (bind _output_get (LocalVariables|SetNew%20Target _besttarget))
    (Utilities|IsValid _output_get
      (:Is%20Valid
        (Utilities|FlowControl|Sequence
          (:then_0
            (TargetLockComponent|EndTargetLock))
          (:then_1
            (TargetLockComponent|SetTargetLockActor (LocalVariables|GetNew%20Target)))
          (:then_2
            (return true))))
      (:Is%20Not%20Valid
        (return false)))
    (else
      (TargetLockComponent|EndTargetLock)
      (return false))))

(fn OnTargetDeath
  (params (Damage :type S%20Damage%20Info%20Structure))
  (TargetLockComponent|EndTargetLock))

(fn GetCameraOrigin
  (bind _camera (Class|BPIwithCamera|GetCameraComponent(Message) (Variables|Default|GetOwnerCharacter)))
  (return _camera))

(fn GetOriginLocation
  (bind _ownercharacter (Variables|Default|GetOwnerCharacter))
  (bind _origin (TargetLockPrivate|GetCameraOrigin))
  (Utilities|IsValid _origin
    (:Is%20Valid
      (return (Transformation|GetWorldLocation _origin) (Transformation|GetWorldRotation _origin)))
    (:Is%20Not%20Valid
      (return (Transformation|GetActorLocation _ownercharacter) (Transformation|GetActorRotation _ownercharacter)))))

(fn SelectBestTargetfromHits
  (params (HitResults :type Array%20of%20Hit%20Result%20Structures))
  (Utilities|FlowControl|Sequence
    (:then_0
      (bind (_location _rotation) (TargetLockPrivate|GetOriginLocation))
      (LocalVariables|SetCone (Utilities|Struct|MakeS_Cone (+ _location (* (Math|Vector|GetForwardVector _rotation) 300)) (Math|Vector|GetForwardVector _rotation) 6e+01 (Variables|Default|GetLockDistance))))
    (:then_1
      (bind _array_element (Utilities|Array|ForEachLoopwithBreak HitResults)
        (:LoopBody
          (bind _islockable (TargetLockPrivate|CheckValidLockTarget (.hitactor _array_element)))
          (if _islockable
            (if (and (.IsInCone (CallFunction|CheckIsinCone (LocalVariables|GetCone) (Transformation|GetActorLocation (.hitactor _array_element)))) (or (< (.DistanceFromCenter (CallFunction|CheckIsinCone (LocalVariables|GetCone) (Transformation|GetActorLocation (.hitactor _array_element)))) (LocalVariables|GetBestDistance)) (< (LocalVariables|GetBestDistance) 0.0)))
              (LocalVariables|SetBestActor (.hitactor _array_element))
              (LocalVariables|SetBestDistance (.DistanceFromCenter (CallFunction|CheckIsinCone (LocalVariables|GetCone) (Transformation|GetActorLocation (.hitactor _array_element))))))))
        (:Completed
          (return (LocalVariables|GetBestActor)))))))

(fn CheckIsTargetVisible
  (Utilities|IsValid (Variables|Default|GetLockTarget)
    (:Is%20Valid
      (bind _location (TargetLockPrivate|GetOriginLocation))
      (LocalVariables|SetOwnerLocation _location)
      (LocalVariables|SetTargetLocation (Transformation|GetActorLocation (Variables|Default|GetLockTarget)))
      (Utilities|FlowControl|Sequence
        (:then_0
          ;[0.15 0.15 0.15 0.5] If too far
          (if (> (Math|Vector|Distance(Vector) (LocalVariables|GetOwnerLocation) (LocalVariables|GetTargetLocation)) (Variables|Default|GetLockDistance))
            (return false)))
        (:then_1
          ;[0.15 0.15 0.15 0.5] If line of sight is broken
          (bind _returnvalue (Collision|LineTraceByChannel (LocalVariables|GetOwnerLocation) (LocalVariables|GetTargetLocation) "TraceTypeQuery1" false (Utilities|Array|MakeArray (Variables|Default|GetOwnerCharacter) (Variables|Default|GetLockTarget)) "None"))
          (if _returnvalue
            (return false)))
        (:then_2
          (return true))))
    (:Is%20Not%20Valid
      (return false))))

(fn TraceTargetLockCone
  (LocalVariables|SetObjects%20to%20Trace (Utilities|Array|MakeArray "ObjectTypeQuery3" "ObjectTypeQuery6" "ObjectTypeQuery5"))
  (bind _location (TargetLockPrivate|GetOriginLocation))
  (bind _outhits (Collision|MultiSphereTraceForObjects _location _location (Variables|Default|GetLockDistance) (LocalVariables|GetObjects%20to%20Trace) false (Utilities|Array|MakeArray (Variables|Default|GetOwnerCharacter)) "None"))
  (bind _besttarget (TargetLockPrivate|SelectBestTargetfromHits _outhits))
  (Utilities|IsValid _besttarget
    (:Is%20Valid
      (return true _besttarget))))

(fn GetControlPitch
  (params (ControllerDesiredPitch :type Float%20%28double-precision%29) (LockAtPitch :type Float%20%28double-precision%29))
  (return (Math|Float|ClampAngle ControllerDesiredPitch (+ LockAtPitch -3e+01) (+ LockAtPitch 15.0))))

(fn UpdateLockTargetPosition
  (bind _ownercharacter (Variables|Default|GetOwnerCharacter))
  (bind _ownercharacter_2 (Variables|Default|GetOwnerCharacter))
  (bind _ownercharacter_3 (Variables|Default|GetOwnerCharacter))
  (bind _returnvalue (AI|GetAIController _ownercharacter_3))
  (bind _returnvalue_2 (Pawn|GetController _ownercharacter))
  (bind _returnvalue_3 (Transformation|GetActorRotation _ownercharacter_2))
  (bind (_islockable _targetlockposition) (Class|BPILockableTarget|GetTargetLockPosition(Message) (Variables|Default|GetLockTarget)))
  (if _islockable
    (LocalVariables|SetOwnerLocation (Transformation|GetActorLocation (Variables|Default|GetOwnerCharacter)))
    (Utilities|FlowControl|Sequence
      (:then_0
        ;[0.15 0.15 0.15 0.5] Lock Camera on target, if player controlled
        (Utilities|IsValid _returnvalue_2
          (:Is%20Valid
            (Pawn|SetControlRotation _returnvalue_2 (Math|Rotator|MakeRotator (.roll (Math|Rotator|FindLookatRotation (LocalVariables|GetOwnerLocation) _targetlockposition)) (TargetLockPrivateMovement|GetControlPitch (.pitch (Pawn|GetDesiredRotation _returnvalue_2)) (.pitch (Math|Rotator|FindLookatRotation (LocalVariables|GetOwnerLocation) _targetlockposition))) (.yaw (Math|Rotator|FindLookatRotation (LocalVariables|GetOwnerLocation) _targetlockposition)))))))
      (:then_1
        ;[0.15 0.15 0.15 0.5] Get coordinates of the place where to lock the actor rotation
        (LocalVariables|SetActorLockLocation (Transformation|GetActorLocation (Variables|Default|GetLockTarget))))
      (:then_2
        ;[0.15 0.15 0.15 0.5] Lock Owner orientation on target
        (bind _result (CallFunction|LockRotationEase _returnvalue_3 (Math|Rotator|FindLookatRotation (LocalVariables|GetOwnerLocation) (LocalVariables|GetActorLockLocation))))
        (Transformation|SetActorRotation (Variables|Default|GetOwnerCharacter) (Math|Rotator|MakeRotator (.roll _result) (.Pitch (Math|Rotator|BreakRotator _returnvalue_3)) (.yaw _result))))
      (:then_3
        ;[0.15 0.15 0.15 0.5] UE doesn't allow to focus pitch on location, only on a pawn. so we focus on acreated tmp pawn
        (Utilities|IsValid _returnvalue
          (:Is%20Valid
            (if (Variables|TargetLockPrivate|GetIsUsePrediction)
              (Utilities|IsValid (Variables|TargetLockPrivate|GetTempFocusPawn)
                (:Is%20Valid
                  (AI|SetFocus _returnvalue (Variables|TargetLockPrivate|GetTempFocusPawn)))
                (:Is%20Not%20Valid
                  (AI|SetFocus _returnvalue (Variables|Default|GetLockTarget) :!label _label)))
              (else
                (goto _label)))))))))

(fn LockRotationEase
  (params (Current :type Rotator) (Target :type Rotator))
  (bind _canrotate (CallFunction|GetCanRotate))
  (if _canrotate
    (return (Math|Interpolation|RInterpTo Current Target (Utilities|Time|GetWorldDeltaSeconds) (CallFunction|GetActorTurnInterpSpeed (Variables|Default|GetOwnerCharacter))))
    (else
      (return Current))))

(fn GetCanRotate
  (return (or (not (Class|Character|IsPlayingRootMotion (Variables|Default|GetOwnerCharacter))) (Variables|/Script/Engine.CharacterMovementComponent|GetbAllowPhysicsRotationDuringAnimRootMotion (Variables|/Script/Engine.Character|GetCharacterMovement (Variables|Default|GetOwnerCharacter))))))

(fn SelectTargetSide
  (params (SideVector :type Vector))
  (bind _locktarget (Variables|Default|GetLockTarget))
  (bind _returnvalue (Transformation|GetActorLocation _locktarget))
  (bind _returnvalue_2 (* SideVector 500))
  (bind _returnvalue_3 (* SideVector 20))
  (bind _returnvalue_4 (+ _returnvalue _returnvalue_2))
  (bind _returnvalue_5 (+ _returnvalue _returnvalue_3))
  (Utilities|IsValid _locktarget
    (:Is%20Valid
      (bind _outhits (Class|KismetSystemLibrary|BoxTraceMultiforObjects _returnvalue_5 _returnvalue_4 "0.000000,500.000000,0.000000" (Math|Rotator|FindLookatRotation _returnvalue_5 _returnvalue_4) (Utilities|Array|MakeArray "ObjectTypeQuery3") false (Utilities|Array|MakeArray (Variables|Default|GetLockTarget) (Variables|Default|GetOwnerCharacter)) "None" true))
      (bind _besttarget (TargetLockPrivate|SelectBestTargetfromHits _outhits))
      (Utilities|IsValid _besttarget
        (:Is%20Valid
          (TargetLockComponent|SetTargetLockActor _besttarget)
          (return true))))
    (:Is%20Not%20Valid
      (return false))))

(fn CheckValidLockTarget
  (params (PossibleTarget :type Object%20Object%20Reference))
  (bind _islockable (Class|BPILockableTarget|GetTargetLockPosition(Message) PossibleTarget))
  (return _islockable))