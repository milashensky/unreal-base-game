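; Attack token component that caps how many melee and ranged attackers can attack at once, using one actor set per type.
; TakeToken picks the set from the drawn weapon, admits newcomers below its cap and lets existing holders continue.
; Each grant restarts a single retriggerable delay, shared by all attackers, that returns the passed actor's token.
; New holders also get an OnDeath binding, and RemoveDeadActors purges dead ones.
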(event Custom|AttackerRefillTick
  (params (Attacking%20Actor :type Actor%20Object%20Reference))
  (Utilities|FlowControl|RetriggerableDelay (Variables|Params|GetBucketRefillDelaySec))
  (AttackTokenComponentPublic|ReturnToken Attacking%20Actor))

(event EventBeginPlay)

(event EventTick
  (params (DeltaSeconds :type Float%20%28single-precision%29)))

(fn TakeToken
  (params (Attacking%20Actor :type Actor%20Object%20Reference))
  (bind _output_get (LocalVariables|SetIsRanged (Private|GetActorRanged Attacking%20Actor)))
  (bind (_canbeattacked _isnew) (CallFunction|CheckCanbeAttackedInternal Attacking%20Actor (select _output_get "NewEnumerator2" "NewEnumerator1")))
  (if _canbeattacked
    (if _isnew
      ;[0.15 0.15 0.15 0.5] If actor is not in the pool yet, add to the correct one based on their weapon and start the timer
      (if (LocalVariables|GetIsRanged)
        (Utilities|Set|Add (Variables|Private|GetRangedActorsBucket) Attacking%20Actor)
        (else
          (Utilities|Set|Add (Variables|Private|GetMeleeActorsBucket) Attacking%20Actor)))
      (Private|StartActorTracking Attacking%20Actor true)
      (return "NewEnumerator1")
      (else
        ;[0.15 0.15 0.15 0.5] If actor is in the pool, they can continue attacking. We just refresh the timer to keep their combo going
        (Private|StartActorTracking Attacking%20Actor false)
        (return "NewEnumerator1")))
    (else
      (return "NewEnumerator2"))))

(fn CheckCanbeAttacked
  (params (Attacking%20actor :type Actor%20Object%20Reference) (Bucket%20Type :type E_AttackTokenBuckets%20Enum :default "NewEnumerator0"))
  (bind _canbeattacked (CallFunction|CheckCanbeAttackedInternal Attacking%20actor Bucket%20Type))
  (if _canbeattacked
    (return "NewEnumerator1")
    (else
      (return "NewEnumerator2"))))

(fn ReturnToken
  (params (Attacking%20Actor :type Actor%20Object%20Reference))
  (Utilities|FlowControl|Sequence
    (:then_0
      (Utilities|Set|Remove (Variables|Private|GetMeleeActorsBucket) Attacking%20Actor))
    (:then_1
      (Utilities|Set|Remove (Variables|Private|GetRangedActorsBucket) Attacking%20Actor))
    (:then_2
      (bind _healthcomponent (Class|PBIDamageable|GetHealthComponent(Message) Attacking%20Actor))
      (Utilities|IsValid _healthcomponent
        (:Is%20Valid
          (EventDispatchers|UnbindEventfromOnDeath _healthcomponent (EventDispatchers|CreateEvent :!event RemoveDeadActors)))))))

(fn GetActorRanged
  (params (Actor :type Actor%20Object%20Reference))
  (bind _drawnweapon (Class|BPIArmed|GetWeaponDawn(Message) Actor))
  (bind _isranged (Class|BPIRangedWeapon|GetIsRanged(Message) _drawnweapon))
  (return _isranged))

(fn StartActorTracking
  (params (Actor :type Actor%20Object%20Reference) (IsNew :type Boolean))
  (Utilities|FlowControl|Sequence
    (:then_0
      (if IsNew
        (bind _healthcomponent (Class|PBIDamageable|GetHealthComponent(Message) Actor))
        (Utilities|IsValid _healthcomponent
          (:Is%20Valid
            (EventDispatchers|BindEventtoOnDeath _healthcomponent (EventDispatchers|CreateEvent :!event RemoveDeadActors))))))
    (:then_1
      (CallFunction|AttackerRefillTick Actor))))

(fn RemoveDeadActors
  (params (Damage :type S%20Damage%20Info%20Structure))
  (Utilities|FlowControl|Sequence
    (:then_0
      (bind _valuepin (Utilities|Set|ForEachLoop(Set) (Variables|Private|GetMeleeActorsBucket))
        (:then
          (Private|ClearifActorDead _valuepin))))
    (:then_1
      (bind _valuepin_2 (Utilities|Set|ForEachLoop(Set) (Variables|Private|GetRangedActorsBucket))
        (:then
          (Private|ClearifActorDead _valuepin_2))))))

(fn ClearifActorDead
  (params (Actor :type Actor%20Object%20Reference%20%28by%20ref%29))
  (bind _isdead (Class|PBIDamageable|GetIsDead(Message) Actor))
  (if _isdead
    (AttackTokenComponentPublic|ReturnToken Actor)))

(fn CheckCanbeAttackedInternal
  (params (Attacking%20Actor :type Actor%20Object%20Reference) (AttackBucketType :type E_AttackTokenBuckets%20Enum :default "NewEnumerator0"))
  (switch Utilities|FlowControl|Switch|SwitchonE_AttackTokenBuckets AttackBucketType
    (:NewEnumerator0
      (bind _enumvalue (|ForEachE_AttackTokenBuckets)
        (:LoopBody
          (if (Utilities|Enum|NotEqual(Enum) _enumvalue "NewEnumerator0")
            (bind (_canbeattacked _isnew) (CallFunction|CheckCanbeAttackedInternal Attacking%20Actor _enumvalue))
            (if _canbeattacked
              (return true _isnew))))
        (:then
          (return false true))))
    (:NewEnumerator1
      (LocalVariables|SetMaxAttackers (Variables|Default|GetMaxAttackingMelee))
      (LocalVariables|SetBucket (Variables|Private|GetMeleeActorsBucket))
      (if (Utilities|Set|Contains (LocalVariables|GetBucket) Attacking%20Actor) :!label _label
        (return true false)
        (else
          (return (< (Utilities|Set|Length (LocalVariables|GetBucket)) (LocalVariables|GetMaxAttackers)) true))))
    (:NewEnumerator2
      (LocalVariables|SetMaxAttackers (Variables|Default|GetMaxAttackingRanged))
      (LocalVariables|SetBucket (Variables|Private|GetRangedActorsBucket))
      (goto _label))))