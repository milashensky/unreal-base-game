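; BPC_SprintWalk is an actor component that switches its owner between walk, run and sprint movement modes.
; Each Start function calls StartNewMode, which ends the previous mode, sets MaxWalkSpeed and replaces the component tags, with dispatchers announcing starts and ends.
; Message calls to the owner supply the movement component and gate sprinting, avoiding casts.
; BeginPlay requests the current mode, so the same-mode check makes it return without applying speed.
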(event EventBeginPlay
  (Variables|Default|SetOwner (Components|GetOwner))
  (switch Utilities|FlowControl|Switch|SwitchonE_WalkMovementMode (Variables|SprintMovementComponent|GetMovementMode)
    (:NewEnumerator1
      (SprintMovementComponent|StartWalk))
    (:NewEnumerator3
      (SprintMovementComponent|StartRun))
    (:NewEnumerator2
      (SprintMovementComponent|StartSprint))))

(fn StartSprint
  (bind _cansprint (Class|BPICanSprint|CheckCanSprint(Message) (Variables|Default|GetOwner)))
  (if _cansprint
    (bind _isset (CallFunction|StartNewMode "NewEnumerator2" (Variables|SprintMovementComponent|GetSprintSpeed)))
    (if _isset
      (Default|CallOnSpintStart))))

(fn StartRun
  (bind _isset (CallFunction|StartNewMode "NewEnumerator3" (Variables|SprintMovementComponent|GetRunSpeed)))
  (if _isset
    (Default|CallOnRunStart)))

(fn StartWalk
  (bind _isset (CallFunction|StartNewMode "NewEnumerator1" (Variables|SprintMovementComponent|GetWalkSpeed)))
  (if _isset
    (Default|CallOnWalkStart)))

(fn EndCurrentMode
  (switch Utilities|FlowControl|Switch|SwitchonE_WalkMovementMode (Variables|SprintMovementComponent|GetMovementMode)
    (:NewEnumerator1
      (Default|CallOnWalkEnd))
    (:NewEnumerator3
      (Default|CallOnRunEnd))
    (:NewEnumerator2
      (Default|CallOnSpintEnd))))

(fn StartNewMode
  (params (NewMode :type E_WalkMovementMode%20Enum :default "NewEnumerator0") (MaxWalkSpeed :type Float%20%28single-precision%29))
  (LocalVariables|SetNewModeLocal NewMode)
  (if (== (Variables|SprintMovementComponent|GetMovementMode) NewMode)
    (return false)
    (else
      (bind _movementcomponent (Class|BPIMovableCharacter|GetCharacterMovementComponent(Message) (Variables|Default|GetOwner)))
      (Utilities|IsValid _movementcomponent
        (:Is%20Valid
          (CallFunction|EndCurrentMode)
          (Variables|/Script/Engine.CharacterMovementComponent|SetMaxWalkSpeed _movementcomponent MaxWalkSpeed)
          (bind _output_get (Variables|SprintMovementComponent|SetMovementMode (LocalVariables|GetNewModeLocal)))
          (Variables|Default|SetComponentTags (Utilities|Array|MakeArray (Utilities|Select :Index _output_get :NewEnumerator0 "Null" :NewEnumerator1 "IsWalking" :NewEnumerator3 "IsRunnung" :NewEnumerator2 "IsSprinting")))
          (return true))
        (:Is%20Not%20Valid
          (return false))))))