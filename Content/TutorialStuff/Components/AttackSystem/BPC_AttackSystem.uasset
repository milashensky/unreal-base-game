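; Actor component that plays combo attacks by cycling through a list of attack montages on the owner's skeletal mesh, fetched by message call.
; Attack refuses while busy; otherwise it plays the current montage, tags the owner "Attacking", advances the index and fires start/end dispatchers.
; Montage notifies end the attack or reset the combo.
; Completion resets all state, with a retriggerable delay as debounced fallback for interrupted attacks.
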(event Custom|PlayAttack
  (bind _skeletalmeshcomponent (Private|GetSkeletalMesh))
  (Utilities|IsValid _skeletalmeshcomponent
    (:Is%20Valid
      (bind _output_get (Variables|Default|SetCurrentAttack (Utilities|Array|Get(acopy) (Variables|AttackComponent|GetAttacks) (Variables|Default|GetAttackIndex))))
      (bind _notifyname (Animation|Montage|PlayMontage _skeletalmeshcomponent (.animation _output_get) (Variables|AttackComponent|GetAttackSpeedRate))
        (:then
          (Variables|AttackComponent|SetIsAttacking true)
          (CallFunction|AddActorTag (Components|GetOwner) "Attacking")
          (Private|SetNextAttackAttack)
          (CallFunction|ScheduleAttackReset (Animation|GetPlayLength (.animation _output_get)))
          (Default|CallOnAttackStart (Variables|Default|GetCurrentAttack)))
        (:OnCompleted
          (AttackComponent|ResetAttackState))
        (:OnInterrupted
          (CallFunction|ScheduleAttackReset 0.5))
        (:OnNotifyBegin
          (switch name _notifyname
            (:AttackEnd
              (Variables|AttackComponent|SetIsAttacking false)
              (Default|CallOnAttackEnd))
            (:ResetCombo
              (AttackComponent|ResetCombo))))))))

(event Custom|ScheduleAttackReset
  (params (Delay :type Float%20%28double-precision%29))
  ;[0.15 0.15 0.15 0.5] Reset Attack state if was knoked out or interrupted otherwise (with debounce)
  (Utilities|FlowControl|RetriggerableDelay (* Delay 1.5))
  (AttackComponent|ResetAttackState))

(event EventBeginPlay)

(event EventTick
  (params (DeltaSeconds :type Float%20%28single-precision%29)))

(fn CheckHasAttacks
  (return (> (Utilities|Array|Length (Variables|AttackComponent|GetAttacks)) 0)))

(fn ResetCombo
  (Variables|Default|SetAttackIndex 0)
  (Variables|Default|SetCurrentAttack ""))

(fn ResetAttackState
  (Utilities|FlowControl|Sequence
    (:then_0
      (if (Variables|AttackComponent|GetIsAttacking)
        (Default|CallOnAttackEnd)))
    (:then_1
      (CallFunction|RemoveActorTag (Components|GetOwner) "Attacking"))
    (:then_2
      (Variables|AttackComponent|SetIsAttacking false))
    (:then_3
      (AttackComponent|ResetCombo))))

(fn CheckCanAttack
  (bind _hasattacks (Private|CheckHasAttacks))
  (return (and _hasattacks (not (Variables|AttackComponent|GetIsAttacking)))))

(fn Attack
  (bind _canattack (AttackComponent|CheckCanAttack))
  (if _canattack
    (CallFunction|PlayAttack)
    (return true)
    (else
      (return false))))

(fn SetNextAttackAttack
  (if (>= (+ (Variables|Default|GetAttackIndex) 1) (Utilities|Array|Length (Variables|AttackComponent|GetAttacks)))
    (Variables|Default|SetAttackIndex 0)
    (else
      (Variables|Default|SetAttackIndex (+ (Variables|Default|GetAttackIndex) 1)))))

(fn GetSkeletalMesh
  (bind _skeletalmeshcomponent (Class|BPIwithSkeletalMeshComponent|GetSkeletalMeshComponent(Message) (Components|GetOwner)))
  (return _skeletalmeshcomponent))